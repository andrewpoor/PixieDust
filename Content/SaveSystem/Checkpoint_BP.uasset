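; Checkpoint actor that reports to the game instance when a Pixie or PlatformerPixie player character walks through it.
; On overlap, its trigger volume disables its collision and calls CheckpointReached on PixieGameInstance.
; The checkpoint ID is parsed from the first actor tag of the form "CPx", and an untagged checkpoint prints an on-screen error at BeginPlay.
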(event OnComponentBeginOverlap(TriggerVolume)
  (params (OverlappedComponent :type Primitive%20Component%20Object%20Reference) (OtherActor :type Actor%20Object%20Reference) (OtherComp :type Primitive%20Component%20Object%20Reference) (OtherBodyIndex :type Integer) (bFromSweep :type Boolean) (SweepResult :type Hit%20Result%20Structure%20%28by%20ref%29))
  (bind _returnvalue (Utilities|GetClass OtherActor))
  ;[1 1 1] If the player walks through this checkpoint, disable it and inform the game instance.
  (if (or (== _returnvalue "/Game/Worlds_Characters/Overworld/OverworldPixieCharacter/Pixie_BP.Pixie_BP_C") (== _returnvalue "/Game/Worlds_Characters/PlatformerWorld/PlatformerPixieCharacter/PlatformerPixie_BP.PlatformerPixie_BP_C"))
    (Collision|SetCollisionEnabled (Variables|Default|GetTrigger%20Volume) "NoCollision")
    (bind _aspixie_game_instance (Utilities|Casting|CastToPixieGameInstance (Game|GetGameInstance)))
    (Default|CheckpointReached _aspixie_game_instance (Math|Conversions|ToInteger(Byte) (Utilities|String|RightChop (Utilities|String|ToString(Name) (Utilities|Array|Get(acopy) (Variables|Actor|GetTags))) 2)))))

(event EventBeginPlay
  (if (not (Utilities|Array|IsValidIndex (Variables|Actor|GetTags))) ; Ensure checkpoint is tagged. If not, this is an error.
    (Development|PrintString (Utilities|String|Append "ERROR: Checkpoint is untagged. Affected CP object: " (Utilities|GetDisplayName self)) true true "(R=0.000000,G=0.660000,B=1.000000,A=1.000000)" 2e+01)))

(event Collision|EventActorBeginOverlap
  (params (OtherActor :type Actor%20Object%20Reference)))

(event EventTick
  (params (DeltaSeconds :type Float%20%28single-precision%29)))

(fn ConstructionScript)