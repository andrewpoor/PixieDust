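; Wingless pixie player character with an isometric follow camera and diagonal-aligned movement.
; BeginPlay computes true isometric pitch from arcsin(1/√3) with 45° yaw, then derives the boom socket offset by trigonometry.
; Input moves along fixed world diagonals, and holding Walk divides the cached running speed.
; Jump and landing set flags for animation, with reset functions for the Animation Blueprint to clear them.
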(event EventBeginPlay
  (bind _cameraboom (Variables|Default|GetCameraBoom))
  (bind _targetarmlength (Variables|/Script/Engine.SpringArmComponent|GetTargetArmLength _cameraboom))
  ;[1 1 1] Set Variables
  (Variables|Movement|SetRunning%20Speed (Variables|/Script/Engine.CharacterMovementComponent|GetMaxWalkSpeed (Variables|Character|GetCharacterMovement)))
  (Variables|Camera|SetCamera%20Pitch (* (Class|KismetMathLibrary|DegAsin (/ 1.0 (Math|Float|Sqrt 3.0))) -1.0)) ; Isometric Pitch Constant
  (Variables|Camera|SetCamera%20Yaw 45.0) ; Isometric Yaw Constant
  ;[1 1 1] Setup Isometric Camera And Movement
  (Transformation|SetWorldRotation (Variables|Default|GetFollowCamera) (Math|Rotator|MakeRotator 0.0 (Variables|Camera|GetCamera%20Pitch) (Variables|Camera|GetCamera%20Yaw)) false false)
  (Variables|/Script/Engine.SpringArmComponent|SetSocketOffset _cameraboom (Math|Vector|MakeVector 0.0 (* (* (Math|Trig|Sin(Degrees) (Variables|Camera|GetCamera%20Yaw)) _targetarmlength) -1.0) (* (Math|Trig|Sin(Degrees) (Math|Float|Absolute(Float) (Variables|Camera|GetCamera%20Pitch))) _targetarmlength))))

(event Collision|EventActorBeginOverlap
  (params (OtherActor :type Actor%20Object%20Reference)))

(event EventTick
  (params (DeltaSeconds :type Float%20%28single-precision%29)))

(event EventOnLanded
  (params (Hit :type Hit%20Result%20Structure%20%28by%20ref%29))
  ;[1 1 1] Jumping Animation Triggers. Toggled off in animation blueprint by calling appropriate functions.
  (Variables|AnimationTriger|SetLanded true))

(event Input|ActionEvents|InputActionJump
  (params (Key :type Key%20Structure))
  ;[1 1 1] Jumping Animation Triggers. Toggled off in animation blueprint by calling appropriate functions.
  (:Pressed
    (Character|Jump)
    (Variables|AnimationTriger|SetJumping true)))

(event Input|ActionEvents|InputActionWalk
  (params (Key :type Key%20Structure))
  (bind _charactermovement (Variables|Character|GetCharacterMovement))
  (bind _running_speed (Variables|Movement|GetRunning%20Speed))
  ;[1 1 1] Switch between walk/run speeds
  (:Pressed
    (Variables|/Script/Engine.CharacterMovementComponent|SetMaxWalkSpeed _charactermovement (/ _running_speed (Variables|Movement|GetWalking%20Speed%20Divisor))))
  (:Released
    (Variables|/Script/Engine.CharacterMovementComponent|SetMaxWalkSpeed _charactermovement _running_speed)))

(event Input|AxisEvents|InputAxisMoveForward
  (params (AxisValue :type Float%20%28single-precision%29))
  (Pawn|Input|AddMovementInput "1.000000,1.000000, 0" AxisValue false))

(event Input|AxisEvents|InputAxisMoveRight
  (params (AxisValue :type Float%20%28single-precision%29))
  (Pawn|Input|AddMovementInput "-1.000000,1.000000, 0" AxisValue false))

(fn ConstructionScript)

(fn ResetAnimJumpTrigger
  (Variables|AnimationTriger|SetJumping false)
  (return))

(fn ResetAnimLandedTrigger
  (Variables|AnimationTriger|SetLanded false)
  (return))