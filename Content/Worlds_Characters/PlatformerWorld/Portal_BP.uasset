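; Level-exit portal for the platformer world that pulls the Pixie player in and opens the next level by name.
; Its trigger zone starts disabled until EnablePortal turns on query collision.
; On overlap it locks player control, hides the HUD, plays a fade-out sequence while a timeline draws the Pixie to its centre, then loads after a delay.
; ClosePortal disables the zone, then spins and scales the portal before destroying it.
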(event Custom|Close%20Portal
  ;[1 1 1] Closes portal to prevent going back in
  (Collision|SetCollisionEnabled (Variables|Default|GetZone) "NoCollision")
  (bind _alpha (Timeline|Portal%20Spins%20And%20Shrinks PlayFromStart)
    (:Update
      (Transformation|SetActorRotation (Math|Rotator|MakeRotator 0.0 (Math|Float|Lerp (Variables|ClosingPortal|GetStarting%20Rotation) (Variables|ClosingPortal|GetEnding%20Rotation) _alpha) 0.0))
      (Transformation|SetActorScale3D (Math|Vector|Lerp(Vector) (Variables|ClosingPortal|GetStarting%20Scale) (Variables|ClosingPortal|GetEnding%20Scale) _alpha)))
    (:Finished
      (Actor|DestroyActor))))

(event Custom|Enable%20Portal
  ;[1 1 1] Allows the player to teleport through the portal on contact
  (Collision|SetCollisionEnabled (Variables|Default|GetZone) "QueryOnly"))

(event EventBeginPlay
  (Variables|ClosingPortal|SetStarting%20Scale (Transformation|GetActorScale3D))
  (Collision|SetCollisionEnabled (Variables|Default|GetZone) "NoCollision"))

(event EventTick
  (params (DeltaSeconds :type Float%20%28single-precision%29)))

(event Collision|EventActorBeginOverlap
  (params (OtherActor :type Actor%20Object%20Reference))
  ;[1 1 1] When player touches the portal, pull them in and then open the next level.
  (bind _asplatformer_pixie_bp (Utilities|Casting|CastToPlatformerPixie_BP OtherActor))
  (Pawn|Components|CharacterMovement|DisableMovement (Variables|/Script/Engine.Character|GetCharacterMovement _asplatformer_pixie_bp))
  (Input|DisableInput _asplatformer_pixie_bp 0)
  (Default|HideHUD _asplatformer_pixie_bp)
  (Variables|EnteringPortal|SetPixie%20Starting%20Location (Transformation|GetActorLocation _asplatformer_pixie_bp))
  (Sequencer|Player|Play (Variables|/Script/LevelSequence.LevelSequenceActor|GetSequencePlayer (Variables|EnteringPortal|GetFade%20Out%20Sequencer)) :!class /Script/MovieScene.MovieSceneSequencePlayer) ; Start fading out
  (bind _alpha (Timeline|Move%20pixie%20to%20centre%20of%20portal PlayFromStart)
    (:Update
      (Transformation|SetActorLocation _asplatformer_pixie_bp (Math|Vector|Lerp(Vector) (Variables|EnteringPortal|GetPixie%20Starting%20Location) (Transformation|GetActorLocation) _alpha) false false) ; Move pixie closer to the centre of the portal
    )
    (:Finished
      (Rendering|SetActorHiddenInGame _asplatformer_pixie_bp true)
      (Audio|PlaySound2D "/Game/Audio/LittleRobotSoundFactory_SFX_Packs/Fantasy/270397__littlerobotsoundfactory__spell-02.270397__littlerobotsoundfactory__spell-02" 1.0 1.0 0.0 0 0)
      (Utilities|FlowControl|Delay (- (Variables|EnteringPortal|GetFade%20Out%20Duration) 0.5)) ; Wait for fade out to finish
      (Game|OpenLevel(byName) (Variables|Default|GetLevel%20Name)))))

(fn ConstructionScript)