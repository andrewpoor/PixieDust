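; Horizontal door prop for the platformer world, a child Blueprint that inherits its door behavior from a parent class.
; On BeginPlay it runs the parent logic, then derives open locations for the top and bottom halves by offsetting their closed locations in opposite directions along X.
; It adds no other logic: overlap and tick events are disabled stubs, and the construction script only calls the parent.
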(event EventBeginPlay
  (|CallParentFunction)
  (Variables|Default|SetTop%20Half%20Open%20Location (+ (Variables|Default|GetTop%20Half%20Closed%20Location) "-19.000000, 0, 0"))
  (Variables|Default|SetBottom%20Half%20Open%20Location (+ (Variables|Default|GetBottom%20Half%20Closed%20Location) "19.000000, 0, 0")))

(event Collision|EventActorBeginOverlap
  (params (OtherActor :type Actor%20Object%20Reference))
  (|CallParentFunction OtherActor) ; This node is disabled and will not be called.\nDrag off pins to build functionality.
)

(event EventTick
  (params (DeltaSeconds :type Float%20%28single-precision%29))
  (|CallParentFunction DeltaSeconds) ; This node is disabled and will not be called.\nDrag off pins to build functionality.
)

(fn ConstructionScript
  (|CallParentFunction))