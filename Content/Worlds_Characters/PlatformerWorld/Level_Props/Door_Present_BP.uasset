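; A platformer level door that opens for the player once they have collected the present.
; When PlatformerPixie_BP overlaps PlayerDetectionBox, it reads CollectedItem from PixieGameInstance and calls DoorOpen if the value matches the expected item.
; DoorOpen is not defined in these graphs, and BeginPlay and Tick are unused.
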(event OnComponentBeginOverlap(PlayerDetectionBox)
  (params (OverlappedComponent :type Primitive%20Component%20Object%20Reference) (OtherActor :type Actor%20Object%20Reference) (OtherComp :type Primitive%20Component%20Object%20Reference) (OtherBodyIndex :type Integer) (bFromSweep :type Boolean) (SweepResult :type Hit%20Result%20Structure%20%28by%20ref%29))
  ;[1 1 1] When player draws near, open if they've collected the present
  (Utilities|Casting|CastToPlatformerPixie_BP OtherActor)
  (bind _aspixie_game_instance (Utilities|Casting|CastToPixieGameInstance (Game|GetGameInstance)))
  (if (Utilities|Enum|Equal(Enum) (Variables|/Game/PixieGameInstance.PixieGameInstance_C|GetCollected%20Item _aspixie_game_instance) "NewEnumerator0")
    (CallFunction|DoorOpen)))

(event EventBeginPlay
  (|CallParentFunction) ; This node is disabled and will not be called.\nDrag off pins to build functionality.
)

(event Collision|EventActorBeginOverlap
  (params (OtherActor :type Actor%20Object%20Reference))
  (|CallParentFunction OtherActor) ; This node is disabled and will not be called.\nDrag off pins to build functionality.
)

(event EventTick
  (params (DeltaSeconds :type Float%20%28single-precision%29))
  (|CallParentFunction DeltaSeconds) ; This node is disabled and will not be called.\nDrag off pins to build functionality.
)

(fn ConstructionScript
  (|CallParentFunction))