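; Platformer box actor that sits in a Docking Switch, toggling its on/off sprite and notifying the switch when inserted or removed.
; Activate removes it and lifts it via a timeline lerp to a pixel-scaled offset.
; PlaceinSwitch snaps it above the assigned switch and lowers it in with a second timeline.
; Collision is disabled while out, and pickup detection returns after a delay only if the switch doesn't clamp the box.
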(event Custom|Place%20in%20Switch
  (bind _docking_switch (Variables|Default|GetDocking%20Switch))
  (bind _docking_switch_2 (Variables|Default|GetDocking%20Switch))
  (bind _returnvalue (Transformation|GetActorLocation _docking_switch))
  (bind (_x _y _z) (Math|Vector|BreakVector _returnvalue))
  ;[1 1 1] Position box over switch
  (bind _output_get (Variables|Default|SetPlaced%20Location (Math|Vector|MakeVector _x (.Y (Math|Vector|BreakVector (Transformation|GetActorLocation))) (+ _z (Variables|Default|GetPixel%20Scale)))))
  (bind _output_get_2 (Variables|Default|SetLifted%20Location (+ _output_get (Variables|Default|GetLifted%20Offset))))
  (Transformation|Teleport _output_get_2 "0, 0, 0")
  ;[1 1 1] Lower into the switch
  (bind _alpha (Timeline|Insert PlayFromStart)
    (:Update
      (Transformation|SetActorLocation (Math|Vector|Lerp(Vector) (Variables|Default|GetLifted%20Location) (Variables|Default|GetPlaced%20Location) _alpha) false true))
    (:Finished
      ;[1 1 1] Set box to 'on', and inform the switch of the box's insertion
      (Default|BoxInserted _docking_switch_2)
      (Collision|SetCollisionEnabled (Variables|Default|GetHitbox) "QueryAndPhysics")
      (if (not (Variables|/Game/Worlds_Characters/PlatformerWorld/Level_Props/Switch_Platformer_BP.Switch_Platformer_BP_C|GetClamps%20Box _docking_switch_2))
        (Utilities|FlowControl|Delay 1.0) ; Wait until door has opened
        (Collision|SetCollisionEnabled (Variables|Default|GetDetection%20Box) "QueryOnly") ; Re-enable pickup detection
        (Rendering|Components|Sprite|SetSprite (Variables|Default|GetPaperSprite) (Variables|Default|GetOn%20Sprite))))))

(event EventBeginPlay
  ;[1 1 1] Setup variables
  (Variables|Default|SetPixel%20Scale (.Z (Math|Vector|BreakVector (Transformation|GetWorldScale (Variables|Default|GetPaperSprite)))))
  (Variables|Default|SetLifted%20Offset (Math|Vector|MakeVector 0.0 0.0 (* (Variables|Default|GetLifted%20Z%20Offset%20In%20Unscaled%20Pixels) (Variables|Default|GetPixel%20Scale))))
  (bind _output_get (Variables|Default|SetPlaced%20Location (Transformation|GetActorLocation)))
  (Variables|Default|SetLifted%20Location (+ _output_get (Variables|Default|GetLifted%20Offset)))
  ;[1 1 1] Set box to 'on', and inform the switch of the box's insertion
  (Rendering|Components|Sprite|SetSprite (Variables|Default|GetPaperSprite) (Variables|Default|GetOn%20Sprite))
  (Utilities|FlowControl|Delay 0.0) ; Wait a frame so everything else can initialise first
  (Default|BoxInserted (Variables|Default|GetDocking%20Switch)))

(event Collision|EventActorBeginOverlap
  (params (OtherActor :type Actor%20Object%20Reference)))

(event EventTick
  (params (DeltaSeconds :type Float%20%28single-precision%29)))

(event EventActivate
  (CallFunction|RemovefromSwitch)
  ;[1 1 1] Lift box out of the switch
  (bind _alpha (Timeline|Rise%20Up PlayFromStart)
    (:Update
      (Transformation|SetActorLocation (Math|Vector|Lerp(Vector) (Variables|Default|GetPlaced%20Location) (Variables|Default|GetLifted%20Location) _alpha) false true))))

(fn ConstructionScript)

(fn RemovefromSwitch
  (Rendering|Components|Sprite|SetSprite (Variables|Default|GetPaperSprite) (Variables|Default|GetOff%20Sprite))
  (Collision|SetCollisionEnabled (Variables|Default|GetDetection%20Box) "NoCollision")
  (Collision|SetCollisionEnabled (Variables|Default|GetHitbox) "NoCollision")
  (Default|BoxRemoved (Variables|Default|GetDocking%20Switch)))