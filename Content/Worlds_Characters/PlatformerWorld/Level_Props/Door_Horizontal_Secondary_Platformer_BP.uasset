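; Horizontal secondary door prop for the platformer world, a child Blueprint that specializes a parent door for sideways-splitting halves.
; On BeginPlay it runs the parent logic, then derives each half's open location by offsetting its closed location in opposite directions along X.
; It then sets the top and bottom holder sprites from the Theme and the Above flag, which only changes the Cloud and Cricket art.
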(event EventBeginPlay
  (|CallParentFunction)
  (Variables|Default|SetTop%20Half%20Open%20Location (+ (Variables|Default|GetTop%20Half%20Closed%20Location) "-19.000000, 0, 0"))
  (Variables|Default|SetBottom%20Half%20Open%20Location (+ (Variables|Default|GetBottom%20Half%20Closed%20Location) "19.000000, 0, 0"))
  (CallFunction|SetSpritesAboveorBelow (Variables|Default|GetTheme) (Variables|Default|GetAbove)))

(event Collision|EventActorBeginOverlap
  (params (OtherActor :type Actor%20Object%20Reference))
  (|CallParentFunction OtherActor) ; This node is disabled and will not be called.\nDrag off pins to build functionality.
)

(event EventTick
  (params (DeltaSeconds :type Float%20%28single-precision%29))
  (|CallParentFunction DeltaSeconds) ; This node is disabled and will not be called.\nDrag off pins to build functionality.
)

(fn ConstructionScript
  (|CallParentFunction))

(fn SetSpritesAboveorBelow
  (params (Theme :type PlatformerTheme%20Enum :default "NewEnumerator0") (Above :type Boolean))
  (Rendering|Components|Sprite|SetSprite (Variables|Default|GetTop%20Holder) (select Above (Utilities|Select :Index Theme :NewEnumerator0 "/Game/Worlds_Characters/PlatformerWorld/Level_Props/Additional_Polish/Space_Door_Holder_Top_Sprite.Space_Door_Holder_Top_Sprite" :NewEnumerator1 "/Game/Worlds_Characters/PlatformerWorld/Level_Props/Additional_Polish/Cloud_Door_Holder_Top_Right_Sprite.Cloud_Door_Holder_Top_Right_Sprite" :NewEnumerator2 "/Game/Worlds_Characters/PlatformerWorld/Level_Props/Additional_Polish/Cricket_Door_Holder_Top_Right_Sprite.Cricket_Door_Holder_Top_Right_Sprite") (Utilities|Select :Index Theme :NewEnumerator0 "/Game/Worlds_Characters/PlatformerWorld/Level_Props/Additional_Polish/Space_Door_Holder_Top_Sprite.Space_Door_Holder_Top_Sprite" :NewEnumerator1 "/Game/Worlds_Characters/PlatformerWorld/Level_Props/Additional_Polish/Cloud_Door_Holder_Top_Left_Sprite.Cloud_Door_Holder_Top_Left_Sprite" :NewEnumerator2 "/Game/Worlds_Characters/PlatformerWorld/Level_Props/Additional_Polish/Cricket_Door_Holder_Top_Left_Sprite.Cricket_Door_Holder_Top_Left_Sprite")))
  (Rendering|Components|Sprite|SetSprite (Variables|Default|GetBottom%20Holder) (select Above (Utilities|Select :Index Theme :NewEnumerator0 "/Game/Worlds_Characters/PlatformerWorld/Level_Props/Additional_Polish/Space_Door_Holder_Bottom_Sprite.Space_Door_Holder_Bottom_Sprite" :NewEnumerator1 "/Game/Worlds_Characters/PlatformerWorld/Level_Props/Additional_Polish/Cloud_Door_Holder_Bottom_Right_Sprite.Cloud_Door_Holder_Bottom_Right_Sprite" :NewEnumerator2 "/Game/Worlds_Characters/PlatformerWorld/Level_Props/Additional_Polish/Cricket_Door_Holder_Bottom_Right_Sprite.Cricket_Door_Holder_Bottom_Right_Sprite") (Utilities|Select :Index Theme :NewEnumerator0 "/Game/Worlds_Characters/PlatformerWorld/Level_Props/Additional_Polish/Space_Door_Holder_Bottom_Sprite.Space_Door_Holder_Bottom_Sprite" :NewEnumerator1 "/Game/Worlds_Characters/PlatformerWorld/Level_Props/Additional_Polish/Cloud_Door_Holder_Bottom_Left_Sprite.Cloud_Door_Holder_Bottom_Left_Sprite" :NewEnumerator2 "/Game/Worlds_Characters/PlatformerWorld/Level_Props/Additional_Polish/Cricket_Door_Holder_Bottom_Left_Sprite.Cricket_Door_Holder_Bottom_Left_Sprite"))))