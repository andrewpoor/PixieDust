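; Sliding two-part sprite door for the platformer world, skinned by a Theme that selects its sprites and click sound.
; DoorOpen and DoorClose adjust a Locks counter, so an open door only closes once the count returns to zero.
; Open and Close timelines lerp the halves vertically apart and back, setting IsOpen when finished.
; The sound is assigned after a short BeginPlay delay so initial positioning at level load stays silent.
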(event Custom|Door%20Close
  (bind _locks (Variables|Default|GetLocks))
  ;[1 1 1] Close the door
  (if (> _locks 0)
    (Math|Integer|DecrementInt _locks
      (:%20%20
        _)))
  (if (and (== _locks 0) (Variables|Default|GetIs%20Open))
    (CallFunction|SlideClosed)
    (Audio|PlaySoundatLocation (Variables|Default|GetOpen/Close%20Sound) (Transformation|GetActorLocation) "0, 0, 0" 1.0 1.0 0.0 0 0 0)))

(event Custom|Door%20Open
  ;[1 1 1] Open the door
  (Math|Integer|IncrementInt (Variables|Default|GetLocks)
    (:%20%20
      (if (not (Variables|Default|GetIs%20Open))
        (CallFunction|SlideOpen)
        (Audio|PlaySoundatLocation (Variables|Default|GetOpen/Close%20Sound) (Transformation|GetActorLocation) "0, 0, 0" 1.0 1.0 0.0 0 0 0)))))

(event Custom|Slide%20Open
  ;[1 1 1] Slide both halves into the ceiling/floor
  (bind _alpha (Timeline|Open PlayFromStart)
    (:Update
      (Transformation|SetRelativeLocation (Variables|Default|GetTop%20Half) (Math|Vector|Lerp(Vector) (Variables|Default|GetTop%20Half%20Closed%20Location) (Variables|Default|GetTop%20Half%20Open%20Location) _alpha) false false)
      (Transformation|SetRelativeLocation (Variables|Default|GetBottom%20Half) (Math|Vector|Lerp(Vector) (Variables|Default|GetBottom%20Half%20Closed%20Location) (Variables|Default|GetBottom%20Half%20Open%20Location) _alpha) false false))
    (:Finished
      (Variables|Default|SetIs%20Open true))))

(event Custom|Slide%20Closed
  ;[1 1 1] Slide both halves back together.
  (bind _alpha (Timeline|Close PlayFromStart)
    (:Update
      (Transformation|SetRelativeLocation (Variables|Default|GetTop%20Half) (Math|Vector|Lerp(Vector) (Variables|Default|GetTop%20Half%20Open%20Location) (Variables|Default|GetTop%20Half%20Closed%20Location) _alpha) false false)
      (Transformation|SetRelativeLocation (Variables|Default|GetBottom%20Half) (Math|Vector|Lerp(Vector) (Variables|Default|GetBottom%20Half%20Open%20Location) (Variables|Default|GetBottom%20Half%20Closed%20Location) _alpha) false false))
    (:Finished
      (Variables|Default|SetIs%20Open false))))

(event EventBeginPlay
  ;[1 1 1] Setup variables
  (bind _output_get (Variables|Default|SetTop%20Half%20Closed%20Location (Variables|/Script/Engine.SceneComponent|GetRelativeLocation (Variables|Default|GetTop%20Half))))
  (Variables|Default|SetTop%20Half%20Open%20Location (+ _output_get "0, 0,19.000000"))
  (bind _output_get_2 (Variables|Default|SetBottom%20Half%20Closed%20Location (Variables|/Script/Engine.SceneComponent|GetRelativeLocation (Variables|Default|GetBottom%20Half))))
  (Variables|Default|SetBottom%20Half%20Open%20Location (+ _output_get_2 "0, 0,-19.000000"))
  ;[1 1 1] Setup door according to theme
  (CallFunction|SetSprites (Variables|Default|GetTheme))
  (Utilities|FlowControl|Delay 2.0) ; Don't play sounds immediately, as some doors open/close to get into position when the level loads
  (Variables|Default|SetOpen/Close%20Sound (Utilities|Select :Index (Variables|Default|GetTheme) :NewEnumerator0 "/Game/Audio/LittleRobotSoundFactory_SFX_Packs/UI/288906__littlerobotsoundfactory__click-mechanical-01.288906__littlerobotsoundfactory__click-mechanical-01" :NewEnumerator1 "/Game/Audio/LittleRobotSoundFactory_SFX_Packs/UI/288910__littlerobotsoundfactory__click-soft-02.288910__littlerobotsoundfactory__click-soft-02" :NewEnumerator2 "/Game/Audio/LittleRobotSoundFactory_SFX_Packs/UI/288907__littlerobotsoundfactory__click-mechanical-00.288907__littlerobotsoundfactory__click-mechanical-00")))

(event Collision|EventActorBeginOverlap
  (params (OtherActor :type Actor%20Object%20Reference)))

(event EventTick
  (params (DeltaSeconds :type Float%20%28single-precision%29)))

(fn ConstructionScript)

(fn SetSprites
  (params (Theme :type PlatformerTheme%20Enum :default "NewEnumerator0"))
  (Rendering|Components|Sprite|SetSprite (Variables|Default|GetTop%20Half) (Utilities|Select :Index Theme :NewEnumerator0 "/Game/Worlds_Characters/PlatformerWorld/Level_Props/Space_Door_Top_Sprite.Space_Door_Top_Sprite" :NewEnumerator1 "/Game/Worlds_Characters/PlatformerWorld/Level_Props/Cloud_Door_Top_Sprite.Cloud_Door_Top_Sprite" :NewEnumerator2 "/Game/Worlds_Characters/PlatformerWorld/Level_Props/Cricket_Door_Top_Sprite.Cricket_Door_Top_Sprite"))
  (Rendering|Components|Sprite|SetSprite (Variables|Default|GetBottom%20Half) (Utilities|Select :Index Theme :NewEnumerator0 "/Game/Worlds_Characters/PlatformerWorld/Level_Props/Space_Door_Bottom_Sprite.Space_Door_Bottom_Sprite" :NewEnumerator1 "/Game/Worlds_Characters/PlatformerWorld/Level_Props/Cloud_Door_Bottom_Sprite.Cloud_Door_Bottom_Sprite" :NewEnumerator2 "/Game/Worlds_Characters/PlatformerWorld/Level_Props/Cricket_Door_Bottom_Sprite.Cricket_Door_Bottom_Sprite"))
  (Rendering|Components|Sprite|SetSprite (Variables|Default|GetTop%20Holder) (Utilities|Select :Index Theme :NewEnumerator0 "/Game/Worlds_Characters/PlatformerWorld/Level_Props/Additional_Polish/Space_Door_Holder_Top_Sprite.Space_Door_Holder_Top_Sprite" :NewEnumerator1 "/Game/Worlds_Characters/PlatformerWorld/Level_Props/Additional_Polish/Cloud_Door_Holder_Top_Sprite.Cloud_Door_Holder_Top_Sprite" :NewEnumerator2 "/Game/Worlds_Characters/PlatformerWorld/Level_Props/Additional_Polish/Cricket_Door_Holder_Top_Sprite.Cricket_Door_Holder_Top_Sprite"))
  (Rendering|Components|Sprite|SetSprite (Variables|Default|GetBottom%20Holder) (Utilities|Select :Index Theme :NewEnumerator0 "/Game/Worlds_Characters/PlatformerWorld/Level_Props/Additional_Polish/Space_Door_Holder_Bottom_Sprite.Space_Door_Holder_Bottom_Sprite" :NewEnumerator1 "/Game/Worlds_Characters/PlatformerWorld/Level_Props/Additional_Polish/Cloud_Door_Holder_Bottom_Sprite.Cloud_Door_Holder_Bottom_Sprite" :NewEnumerator2 "/Game/Worlds_Characters/PlatformerWorld/Level_Props/Additional_Polish/Cricket_Door_Holder_Bottom_Sprite.Cricket_Door_Holder_Bottom_Sprite")))