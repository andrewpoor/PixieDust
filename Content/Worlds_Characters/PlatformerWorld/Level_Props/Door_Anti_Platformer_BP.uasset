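; An inverted platformer door that starts open and closes when enough Door Open requests accumulate.
; Door Open increments a lock count and slides the door shut once it reaches the required number.
; Door Close decrements the count and slides the door open again when it falls below that threshold.
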(event EventBeginPlay
  ;[1 1 1] Door starts open.
  (|CallParentFunction)
  (CallFunction|SlideOpen))

(event EventDoorOpen
  ;[1 1 1] When 'Door Open' is called, this door *closes*, though only when it has been asked to close a sufficient number of times.
  (bind _result (Math|Integer|IncrementInt (Variables|Default|GetLocks))
    (:%20%20
      (if (and (>= _result (Variables|Default|GetLocks%20Required)) (Variables|Default|GetIs%20Open))
        (CallFunction|SlideClosed)))))

(event EventDoorClose
  ;[1 1 1] When 'Door Close' is called, this door *opens*.
  (bind _result (Math|Integer|DecrementInt (Variables|Default|GetLocks))
    (:%20%20
      (if (and (< _result (Variables|Default|GetLocks%20Required)) (not (Variables|Default|GetIs%20Open)))
        (CallFunction|SlideOpen)))))

(fn ConstructionScript
  (|CallParentFunction))