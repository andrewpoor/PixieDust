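; Platformer switch actor that opens and closes its linked doors when a box is inserted or removed.
; It shows the off sprite on BeginPlay.
; BoxInserted disables the Box component's collision, shows the on sprite and calls DoorOpen on each of the ConnectedDoors.
; BoxRemoved restores query-only collision, reverts the sprite and calls DoorClose; neither function is called within this Blueprint.
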(event EventBeginPlay
  (Rendering|Components|Sprite|SetSprite (Variables|Default|GetPaperSprite) (Variables|Default|GetOff%20Sprite)))

(event Collision|EventActorBeginOverlap
  (params (OtherActor :type Actor%20Object%20Reference)))

(event EventTick
  (params (DeltaSeconds :type Float%20%28single-precision%29)))

(fn ConstructionScript)

(fn BoxRemoved
  (Collision|SetCollisionEnabled (Variables|Default|GetBox) "QueryOnly")
  (Rendering|Components|Sprite|SetSprite (Variables|Default|GetPaperSprite) (Variables|Default|GetOff%20Sprite))
  (for _array_element (Variables|Default|GetConnected%20Doors)
    (Default|DoorClose _array_element)))

(fn BoxInserted
  (Collision|SetCollisionEnabled (Variables|Default|GetBox) "NoCollision")
  (Rendering|Components|Sprite|SetSprite (Variables|Default|GetPaperSprite) (Variables|Default|GetOn%20Sprite))
  (for _array_element (Variables|Default|GetConnected%20Doors)
    (Default|DoorOpen _array_element)))