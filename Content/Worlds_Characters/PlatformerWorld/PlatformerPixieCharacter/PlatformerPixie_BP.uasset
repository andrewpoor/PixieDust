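; Player pixie character for a 2D side-scrolling platformer that runs, jumps, teleports to a placed magic circle and carries boxes into switches.
; Tick picks idle, run or midair flipbooks, with holding variants, unless jump, landing or FlipbookBusy actions own the sprite.
; Spell and object actions mostly disable input for delays timed to flipbook length; forward line traces find boxes and switches.
; Teleporting corrects drift off the Y plane; BeginPlay creates the HUD.
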(event EventBeginPlay
  (Components|Timeline|SetLooping (Variables|Default|GetSprite) false)
  (Variables|Default|SetDefault%20Y%20Position (.Y (Math|Vector|BreakVector (Transformation|GetActorLocation))))
  ;[1 1 1] Display UI
  (bind _returnvalue (UserInterface|CreateWidget "/Game/UI/PlatformerPixieHUD.PlatformerPixieHUD_C"))
  (bind _output_get (Variables|Default|SetHUD _returnvalue))
  (UserInterface|Viewport|AddtoViewport _output_get 0))

(event Collision|EventActorBeginOverlap
  (params (OtherActor :type Actor%20Object%20Reference)))

(event EventTick
  (params (DeltaSeconds :type Float%20%28single-precision%29))
  (bind _holding_object (Variables|Default|GetHolding%20Object))
  (bind _sprite (Variables|Default|GetSprite))
  (bind _sprite_2 (Variables|Default|GetSprite))
  ;[1 1 1] Manage running and idle animations
  (if (not (Math|Boolean|ORBoolean (Variables|Movement|GetJumping) (Variables|Movement|GetLanded) (Variables|Default|GetFlipbook%20Busy)))
    (if (AI|Components|NavMovement|IsFalling (Variables|Character|GetCharacterMovement))
      (Sprite|SetFlipbook _sprite_2 (select (Variables|Default|GetHolding%20Object) "/Game/Worlds_Characters/PlatformerWorld/PlatformerPixieCharacter/Sprites/Flipbooks/Pixie_Holding_Object_Midair_Flipbook.Pixie_Holding_Object_Midair_Flipbook" "/Game/Worlds_Characters/PlatformerWorld/PlatformerPixieCharacter/Sprites/Flipbooks/Pixie_Midair_Flipbook.Pixie_Midair_Flipbook")) ; Midair
      (else
        (if (Variables|Movement|GetRunning)
          (Sprite|SetFlipbook _sprite_2 (select _holding_object "/Game/Worlds_Characters/PlatformerWorld/PlatformerPixieCharacter/Sprites/Flipbooks/Pixie_Holding_Object_Running_Flipbook.Pixie_Holding_Object_Running_Flipbook" "/Game/Worlds_Characters/PlatformerWorld/PlatformerPixieCharacter/Sprites/Flipbooks/Pixie_Run_Flipbook.Pixie_Run_Flipbook")) ; Running
          (else
            (Sprite|SetFlipbook _sprite_2 (select _holding_object "/Game/Worlds_Characters/PlatformerWorld/PlatformerPixieCharacter/Sprites/Flipbooks/Pixie_Holding_Object_Idle_Flipbook.Pixie_Holding_Object_Idle_Flipbook" "/Game/Worlds_Characters/PlatformerWorld/PlatformerPixieCharacter/Sprites/Flipbooks/Pixie_Idle_Flipbook.Pixie_Idle_Flipbook")) ; Idle
          ))
        (Components|Timeline|SetLooping _sprite true)
        (Audio|Components|Audio|Play _sprite)))))

(event EventOnLanded
  (params (Hit :type Hit%20Result%20Structure%20%28by%20ref%29))
  (bind _sprite (Variables|Default|GetSprite))
  ;[1 1 1] Player jumping
  (Audio|PlaySound2D "/Game/Audio/LittleRobotSoundFactory_SFX_Packs/Fantasy/270416__littlerobotsoundfactory__footstep-dirt-07.270416__littlerobotsoundfactory__footstep-dirt-07" 1.0 1.0 0.0 0 0)
  (Variables|Movement|SetJumping false)
  (Variables|Movement|SetLanded true)
  (Sprite|SetFlipbook _sprite (select (Variables|Default|GetHolding%20Object) "/Game/Worlds_Characters/PlatformerWorld/PlatformerPixieCharacter/Sprites/Flipbooks/Pixie_Holding_Object_Land_Flipbook.Pixie_Holding_Object_Land_Flipbook" "/Game/Worlds_Characters/PlatformerWorld/PlatformerPixieCharacter/Sprites/Flipbooks/Pixie_Land_Flipbook.Pixie_Land_Flipbook"))
  (Audio|Components|Audio|Play _sprite)
  (Utilities|FlowControl|RetriggerableDelay (Class|PaperFlipbookComponent|GetFlipbookLength _sprite))
  (Variables|Movement|SetLanded false))

(event Input|ActionEvents|InputActionJump
  (params (Key :type Key%20Structure))
  (bind _sprite (Variables|Default|GetSprite))
  ;[1 1 1] Player jumping
  (:Pressed
    (if (not (AI|Components|NavMovement|IsFalling (Variables|Character|GetCharacterMovement)))
      (Audio|PlaySound2D "/Game/Audio/LittleRobotSoundFactory_SFX_Packs/8-Bit/270337__littlerobotsoundfactory__pickup-00.270337__littlerobotsoundfactory__pickup-00" 1.0 1.0 0.0 0 0)
      (Character|Jump)
      (Variables|Movement|SetJumping true)
      (Sprite|SetFlipbook _sprite (select (Variables|Default|GetHolding%20Object) "/Game/Worlds_Characters/PlatformerWorld/PlatformerPixieCharacter/Sprites/Flipbooks/Pixie_Holding_Object_Jump_Flipbook.Pixie_Holding_Object_Jump_Flipbook" "/Game/Worlds_Characters/PlatformerWorld/PlatformerPixieCharacter/Sprites/Flipbooks/Pixie_Jump_Flipbook.Pixie_Jump_Flipbook"))
      (Components|Timeline|SetLooping _sprite false)
      (Audio|Components|Audio|Play (Variables|Default|GetSprite)))))

(event Input|ActionEvents|InputActionPlaceMagicCircle
  (params (Key :type Key%20Structure))
  (bind _sprite (Variables|Default|GetSprite))
  ;[1 1 1] Place Magic Circle
  (:Pressed
    (if (not (or (Variables|Default|GetHolding%20Object) (AI|Components|NavMovement|IsFalling (Variables|Character|GetCharacterMovement))))
      (Input|DisableInput 0)
      (Variables|Default|SetFlipbook%20Busy true)
      (Sprite|SetFlipbook _sprite "/Game/Worlds_Characters/PlatformerWorld/PlatformerPixieCharacter/Sprites/Flipbooks/Pixie_Place_Circle_Flipbook.Pixie_Place_Circle_Flipbook")
      (Utilities|FlowControl|Delay (/ (Class|PaperFlipbookComponent|GetFlipbookLength _sprite) 2.0))
      (if (Utilities|IsValid (Variables|Default|GetMagic%20Circle)) ; If a circle doesn't exist yet, spawn one
        _
        (else
          (bind _returnvalue (Game|SpawnActorfromClass "/Game/Worlds_Characters/PlatformerWorld/Magic_Circle_Platformer/2D_Magic_Circle_BP.2D_Magic_Circle_BP_C" (Transformation|GetActorTransform) "Undefined" 0 0))
          (Variables|Default|SetMagic%20Circle _returnvalue)))
      (Transformation|Teleport (Variables|Default|GetMagic%20Circle) (+ (Transformation|GetActorLocation) (Variables|Default|GetMagic%20Circle%20Offset)) "0, 0, 0") ; Move the circle under the player
      (Audio|PlaySound2D "/Game/Audio/LittleRobotSoundFactory_SFX_Packs/Fantasy/270409__littlerobotsoundfactory__spell-00.270409__littlerobotsoundfactory__spell-00" 1.0 1.0 0.0 0 0)
      (Utilities|FlowControl|Delay (/ (Class|PaperFlipbookComponent|GetFlipbookLength (Variables|Default|GetSprite)) 2.0))
      (Variables|Default|SetFlipbook%20Busy false)
      (Input|EnableInput 0))))

(event Input|ActionEvents|InputActionTeleportSpell
  (params (Key :type Key%20Structure))
  (bind _returnvalue (Transformation|GetActorLocation))
  (bind _sprite (Variables|Default|GetSprite))
  (bind _sprite_2 (Variables|Default|GetSprite))
  (bind (_x _y _z) (Math|Vector|BreakVector _returnvalue))
  ;[1 1 1] Cast Teleport Spell
  (:Pressed
    (if (Utilities|IsValid (Variables|Default|GetMagic%20Circle)) ; Only teleport if circle exists
      (Input|DisableInput 0)
      (Variables|Default|SetFlipbook%20Busy true)
      (Sprite|SetFlipbook _sprite (select (Variables|Default|GetHolding%20Object) "/Game/Worlds_Characters/PlatformerWorld/PlatformerPixieCharacter/Sprites/Flipbooks/Pixie_Holding_Object_Idle_Flipbook.Pixie_Holding_Object_Idle_Flipbook" "/Game/Worlds_Characters/PlatformerWorld/PlatformerPixieCharacter/Sprites/Flipbooks/Pixie_Start_Teleport_Flipbook.Pixie_Start_Teleport_Flipbook"))
      (Utilities|FlowControl|Delay (* (Class|PaperFlipbookComponent|GetFlipbookLength _sprite) 0.9))
      (Transformation|Teleport (- (Transformation|GetActorLocation (Variables|Default|GetMagic%20Circle)) (Variables|Default|GetMagic%20Circle%20Offset)) "0, 0, 0")
      (Audio|PlaySound2D "/Game/Audio/LittleRobotSoundFactory_SFX_Packs/Fantasy/270396__littlerobotsoundfactory__spell-01.270396__littlerobotsoundfactory__spell-01" 1.0 1.0 0.0 0 0)
      (Sprite|SetFlipbook _sprite_2 (select (Variables|Default|GetHolding%20Object) "/Game/Worlds_Characters/PlatformerWorld/PlatformerPixieCharacter/Sprites/Flipbooks/Pixie_Holding_Object_Idle_Flipbook.Pixie_Holding_Object_Idle_Flipbook" "/Game/Worlds_Characters/PlatformerWorld/PlatformerPixieCharacter/Sprites/Flipbooks/Pixie_End_Teleport_Flipbook.Pixie_End_Teleport_Flipbook"))
      (Utilities|FlowControl|Delay (* (Class|PaperFlipbookComponent|GetFlipbookLength _sprite_2) 0.9))
      (if (> (Math|Float|Absolute(Float) _y) (+ (Variables|Default|GetDefault%20Y%20Position) 0.2)) ; Check if something has pushed the player out in the Y direction
        (Transformation|SetActorLocation (Math|Vector|MakeVector (+ _x 2e+01) (Variables|Default|GetDefault%20Y%20Position) _z) false false) ; Set the player back to the correct Y position and move them past whatever was pushing them.
      )
      (Variables|Default|SetFlipbook%20Busy false)
      (Input|EnableInput 0))))

(event Input|ActionEvents|InputActionActivateObject
  (params (Key :type Key%20Structure))
  (bind _returnvalue (Transformation|GetActorLocation))
  (bind _returnvalue_2 (Transformation|GetActorLocation))
  (bind _sprite (Variables|Default|GetSprite))
  (bind _returnvalue_3 (Class|PaperFlipbookComponent|GetFlipbookLength _sprite))
  (bind _returnvalue_4 (* _returnvalue_3 0.95))
  ;[1 1 1] Pick up or put down an object (such as a box)
  (:Pressed
    (if (not (AI|Components|NavMovement|IsFalling (Variables|Character|GetCharacterMovement)))
      (if (Variables|Default|GetHolding%20Object)
        ;;[1 1 1] Try to Place the Object in a Switch
        (bind (_outhit _returnvalue_5) (Collision|LineTraceByChannel _returnvalue (+ _returnvalue (* (Transformation|GetActorForwardVector) (Variables|Default|GetActivate%20Trace%20Distance))) "TraceTypeQuery3" false 0 "None")) ; Check if switch in front
        (if _returnvalue_5
          (bind _asswitch_platformer_bp (Utilities|Casting|CastToSwitch_Platformer_BP (.HitActor (Collision|BreakHitResult _outhit)))) ; If switch, place box in it. Otherwise do nothing.
          (Transformation|DetachFromActor (Variables|Default|GetHeld%20Object) "KeepWorld" "KeepWorld" "KeepWorld")
          (Variables|Default|SetHolding%20Object false)
          (Variables|/Game/Worlds_Characters/PlatformerWorld/Level_Props/Box_Platformer_BP.Box_Platformer_BP_C|SetDocking%20Switch (Variables|Default|GetHeld%20Object) _asswitch_platformer_bp)
          (Default|PlaceinSwitch (Variables|Default|GetHeld%20Object))
          ;;;[1 1 1] Play 'lowering arms' animation
          (Input|DisableInput 0)
          (Variables|Default|SetFlipbook%20Busy true)
          (Sprite|SetFlipbook (Variables|Default|GetSprite) "/Game/Worlds_Characters/PlatformerWorld/PlatformerPixieCharacter/Sprites/Flipbooks/Pixie_Reach_Back_Flipbook.Pixie_Reach_Back_Flipbook")
          (Utilities|FlowControl|Delay (* (Class|PaperFlipbookComponent|GetFlipbookLength (Variables|Default|GetSprite)) 0.9)) ; Wait for 'lower arms' animation to finish
          (Audio|PlaySound2D "/Game/Audio/LittleRobotSoundFactory_SFX_Packs/8-Bit/270338__littlerobotsoundfactory__open-01.270338__littlerobotsoundfactory__open-01" 1.0 1.0 0.0 0 0)
          (Variables|Default|SetFlipbook%20Busy false)
          (Input|EnableInput 0))
        (else
          ;;[1 1 1] Try to Pick up an Object
          (Input|DisableInput 0)
          (Variables|Default|SetFlipbook%20Busy true)
          (Sprite|SetFlipbook (Variables|Default|GetSprite) "/Game/Worlds_Characters/PlatformerWorld/PlatformerPixieCharacter/Sprites/Flipbooks/Pixie_Reach_Out_Flipbook.Pixie_Reach_Out_Flipbook")
          (bind (_outhit_2 _returnvalue_6) (Collision|LineTraceByChannel _returnvalue_2 (+ _returnvalue_2 (* (Transformation|GetActorForwardVector) (Variables|Default|GetActivate%20Trace%20Distance))) "TraceTypeQuery3" false 0 "None")) ; Check if object in front
          (if _returnvalue_6
            (bind _asbox_platformer_bp (Utilities|Casting|CastToBox_Platformer_BP (.HitActor (Collision|BreakHitResult _outhit_2)))
              (:then
                ;;;[1 1 1] If there is an object, pick it up.
                (bind _output_get (Variables|Default|SetHeld%20Object _asbox_platformer_bp))
                (Class|ActivatableI|Activate(Message) _output_get)
                (Audio|PlaySound2D "/Game/Audio/LittleRobotSoundFactory_SFX_Packs/8-Bit/270338__littlerobotsoundfactory__open-01.270338__littlerobotsoundfactory__open-01" 1.0 1.0 0.0 0 0)
                (Utilities|FlowControl|Delay _returnvalue_4) ; Wait for 'raise arms' animation to finish
                (Transformation|AttachActorToActor (Variables|Default|GetHeld%20Object) self "None" "KeepWorld" "KeepWorld" "KeepWorld" true)
                (Transformation|SetActorLocation (Variables|Default|GetHeld%20Object) (+ (Transformation|GetActorLocation) (* (Variables|Default|GetHeld%20Object%20Offset) (+ (Transformation|GetActorForwardVector) (Transformation|GetActorUpVector)))) false true) ; Nudge the held object closer to the player
                (Variables|Default|SetHolding%20Object true)
                (Variables|Default|SetFlipbook%20Busy false)
                (Input|EnableInput 0))
              (:CastFailed
                ;;;[1 1 1] If there's no object, lower arms and finish the animation.
                (Utilities|FlowControl|Delay _returnvalue_4 :!label _label) ; Wait for 'raise arms' animation to finish
                (Sprite|SetFlipbook (Variables|Default|GetSprite) "/Game/Worlds_Characters/PlatformerWorld/PlatformerPixieCharacter/Sprites/Flipbooks/Pixie_Reach_Back_Flipbook.Pixie_Reach_Back_Flipbook")
                (Utilities|FlowControl|Delay (* (Class|PaperFlipbookComponent|GetFlipbookLength (Variables|Default|GetSprite)) 0.9)) ; Wait for 'lower arms' animation to finish
                (Variables|Default|SetFlipbook%20Busy false)
                (Input|EnableInput 0)))
            (else
              (goto _label))))))))

(event Input|AxisEvents|InputAxisMoveRight
  (params (AxisValue :type Float%20%28single-precision%29))
  ;[1 1 1] Player left/right movement
  (Variables|Movement|SetRunning (> (Math|Float|Absolute(Float) AxisValue) 0.05))
  (Pawn|Input|AddMovementInput "1.000000,0.000000, 0" AxisValue false)
  (Math|Float|CompareFloat AxisValue 0.0 ; Get Facing Direction
    (:>
      (Pawn|SetControlRotation (Pawn|GetController) (Math|Rotator|MakeRotator 0.0 0.0 0.0)))
    (:<
      (Pawn|SetControlRotation (Pawn|GetController) (Math|Rotator|MakeRotator 0.0 0.0 1.8e+02)))))

(fn ConstructionScript)

(fn SetLooping
  (params (Looping :type Boolean))
  (bind _sprite (Variables|Default|GetSprite))
  (Components|Timeline|SetLooping _sprite Looping)
  (if (and Looping (not (Audio|Components|Audio|IsPlaying _sprite)))
    (Audio|Components|Audio|Play (Variables|Default|GetSprite))
    (return)))

(fn HideHUD
  (Widget|SetVisibility (Variables|Default|GetHUD) "Hidden"))