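; Player pixie character for the overworld that floats, drops and flies using limited jump boosts refilled on landing.
; Tick zeroes gravity beyond the current falling speed to cap descent.
; Timed, input-locking actions place a magic circle, teleport to it and line-trace to activate objects.
; It also manages its HUD, scripted launches and cutscene input, dispatching scanner and present-pickup cutscenes to the level blueprint.
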(event Custom|Launch%20Pixie
  (params (Launch%20Velocity :type Vector) (Flight%20Duration :type Float%20%28single-precision%29) (Align%20With%20Velocity :type Boolean) (Reenable%20Input :type Boolean))
  ;[1 1 1] When the bin lid flips open, the player is launched up into the air.
  (Variables|/Script/Engine.CharacterMovementComponent|SetFallingLateralFriction (Variables|Character|GetCharacterMovement) (Variables|LaunchingFromBin|GetLaunching%20Lateral%20Friction))
  (Variables|Movement|SetFalling%20Speed (Variables|LaunchingFromBin|GetLaunching%20Falling%20Speed))
  (if Align%20With%20Velocity
    (Pawn|SetControlRotation (Pawn|GetController) (Transformation|GetWorldRotation (Variables|Default|GetCapsuleComponent))) ; Face camera behind pixie
  )
  (Input|DisableInput 0)
  (Character|LaunchCharacter Launch%20Velocity true true)
  (Variables|AnimationTrigger|SetFlyBoost true) ; Trigger flying animation
  (Utilities|FlowControl|Delay 0.01)
  (Variables|AnimationTrigger|SetFlyBoost false)
  (Utilities|FlowControl|Delay Flight%20Duration)
  (Variables|/Script/Engine.CharacterMovementComponent|SetFallingLateralFriction (Variables|Character|GetCharacterMovement) (Variables|LaunchingFromBin|GetDefault%20Lateral%20Friction))
  (Variables|Movement|SetFalling%20Speed (Variables|Movement|GetFloating%20Speed))
  (if Reenable%20Input ; Reenable input if necessary
    (Input|EnableInput 0)))

(event Custom|Cutscene%20Start
  ;[1 1 1] Disable player input for a cinematic cutscene until it's over.
  (Input|DisableInput 0)
  (Widget|SetVisibility (Variables|Default|GetHUD) "Hidden"))

(event Custom|Cutscene%20Finished
  ;[1 1 1] Once a cutscene is over, restore control to the player.
  (Input|EnableInput 0)
  (Widget|SetVisibility (Variables|Default|GetHUD) "Visible"))

(event Custom|Pickup%20Present
  ;[1 1 1] Pick up present
  (Default|ItemCollected (Variables|Default|GetHUD) "NewEnumerator0")
  (bind _aspixie_game_instance (Utilities|Casting|CastToPixieGameInstance (Game|GetGameInstance)))
  (Variables|/Game/PixieGameInstance.PixieGameInstance_C|SetCollected%20Item _aspixie_game_instance "NewEnumerator0")
  (Default|CallStartLookatParentCutscene) ; Dispatch event to level blueprint
)

(event EventBeginPlay
  ;[1 1 1] Set variables
  (Variables|Movement|SetFalling%20Speed (Variables|Movement|GetFloating%20Speed)) ; Default falling speed is floating gently downwards
  (Variables|Movement|SetGravity%20Scale (Variables|Movement|GetFloating%20Gravity))
  (Variables|Movement|SetRunning%20Speed (Variables|/Script/Engine.CharacterMovementComponent|GetMaxWalkSpeed (Variables|Character|GetCharacterMovement)))
  (Variables|Default|SetFlight%20Boosts%20Remaining (Variables|Default|GetTotal%20Flight%20Boosts))
  (Variables|Ability|SetMagic%20Circle%20Offset (- (Components|Capsule|GetScaledCapsuleHalfHeight (Variables|Default|GetCapsuleComponent)) (Variables|Ability|GetMagic%20Circle%20Ground%20Offset)))
  (Variables|LaunchingFromBin|SetDefault%20Lateral%20Friction (Variables|/Script/Engine.CharacterMovementComponent|GetFallingLateralFriction (Variables|Character|GetCharacterMovement)))
  ;[1 1 1] Display UI
  (bind _returnvalue (UserInterface|CreateWidget "/Game/UI/OverworldPixieHUD.OverworldPixieHUD_C"))
  (bind _output_get (Variables|Default|SetHUD _returnvalue))
  (UserInterface|Viewport|AddtoViewport _output_get 0)
  ;[1 1 1] Apply Control Settings
  (bind _returnvalue_2 (UserInterface|CreateWidget "/Game/UI/ControlsMenu_BP.ControlsMenu_BP_C"))
  (Default|LoadSettings _returnvalue_2)
  (Default|ApplySettings _returnvalue_2))

(event Collision|EventActorBeginOverlap
  (params (OtherActor :type Actor%20Object%20Reference)))

(event EventTick
  (params (DeltaSeconds :type Float%20%28single-precision%29))
  (bind _charactermovement (Variables|Character|GetCharacterMovement))
  ;[1 1 1] Adjust falling speed
  (if (< (.Z (Math|Vector|BreakVector (Transformation|GetVelocity))) (* (Variables|Movement|GetFalling%20Speed) -1.0)) ; If falling too fast:
    (Variables|/Script/Engine.CharacterMovementComponent|SetGravityScale _charactermovement 0.0)
    (else
      (Variables|/Script/Engine.CharacterMovementComponent|SetGravityScale _charactermovement (Variables|Movement|GetGravity%20Scale)))))

(event EventOnLanded
  (params (Hit :type Hit%20Result%20Structure%20%28by%20ref%29))
  ;[1 1 1] Fly by repeatedly jumping
  (Variables|Movement|SetCan%20Jump true)
  (Variables|Default|SetFlight%20Boosts%20Remaining (Variables|Default|GetTotal%20Flight%20Boosts))
  (Default|ResetFlightBoosts (Variables|Default|GetHUD))
  (Utilities|FlowControl|DoN (Variables|Default|GetTotal%20Flight%20Boosts)) ; enters at Reset
)

(event Input|ActionEvents|InputActionDrop
  (params (Key :type Key%20Structure))
  (bind _charactermovement (Variables|Character|GetCharacterMovement))
  ;[1 1 1] Drop on command
  (:Pressed
    (if (Variables|Default|GetIs%20Accepting%20Inputs)
      (Variables|Movement|SetFalling%20Speed (Variables|Movement|GetDropping%20Speed))
      (Variables|Movement|SetGravity%20Scale (Variables|Movement|GetDropping%20Gravity))
      (Variables|AnimationTrigger|SetDropping true)))
  (:Released
    (Variables|Movement|SetFalling%20Speed (Variables|Movement|GetFloating%20Speed))
    (Variables|Movement|SetGravity%20Scale (Variables|Movement|GetFloating%20Gravity))
    (Variables|AnimationTrigger|SetDropping false)
    (if (AI|Components|NavMovement|IsFalling _charactermovement) ; If still falling, cut momentum.
      (Components|Movement|StopMovementImmediately _charactermovement))))

(event Input|ActionEvents|InputActionJump
  (params (Key :type Key%20Structure))
  ;[1 1 1] Fly by repeatedly jumping
  (:Pressed
    ;;[1 1 1] While jump is held, loop until "you can jump" conditions are true. If jump is released, exit loop.
    (bind _output_get (Variables|Movement|SetJump%20Held true))
    (if _output_get :!label _label
      (if (Math|Boolean|ANDBoolean (Variables|Movement|GetCan%20Jump) (Variables|Default|GetIs%20Accepting%20Inputs) (not (Variables|AnimationTrigger|GetDropping)))
        (Variables|Movement|SetJump%20Held false)
        (if (AI|Components|NavMovement|IsFalling (Variables|Character|GetCharacterMovement)) ; If not on the ground, use a 'flight boost'. Otherwise jump.
          (Utilities|FlowControl|DoN (Variables|Default|GetTotal%20Flight%20Boosts)
            (:Exit
              (Math|Integer|DecrementInt (Variables|Default|GetFlight%20Boosts%20Remaining)
                (:%20%20
                  (Default|FlightBoostUsed (Variables|Default|GetHUD))
                  (Character|LaunchCharacter (Math|Vector|MakeVector 0.0 0.0 (Variables|/Script/Engine.CharacterMovementComponent|GetJumpZVelocity (Variables|Character|GetCharacterMovement))) false true) ; "Flight boost"
                  (Variables|Movement|SetCan%20Jump false)
                  (Variables|AnimationTrigger|SetFlyBoost true)
                  (Utilities|FlowControl|Delay 0.0)
                  (Variables|AnimationTrigger|SetFlyBoost false)))))
          (else
            (Character|Jump)
            (Variables|Movement|SetCan%20Jump false)
            (Variables|AnimationTrigger|SetJumping true)
            (Utilities|FlowControl|Delay 0.0)
            (Variables|AnimationTrigger|SetJumping false)))
        (Utilities|FlowControl|Delay (Variables|Movement|GetFlight%20Boost%20Delay))
        (Variables|Movement|SetCan%20Jump true)
        (else
          (Utilities|FlowControl|Delay 0.0) ; Skip to next frame
          (goto _label)))))
  (:Released
    (Variables|Movement|SetJump%20Held false)))

(event Input|ActionEvents|InputActionWalk
  (params (Key :type Key%20Structure))
  (bind _charactermovement (Variables|Character|GetCharacterMovement))
  (bind _running_speed (Variables|Movement|GetRunning%20Speed))
  ;[1 1 1] Switch between walk/run speeds
  (:Pressed
    (Variables|/Script/Engine.CharacterMovementComponent|SetMaxWalkSpeed _charactermovement (/ _running_speed (Variables|Movement|GetWalking%20Speed%20Divisor))))
  (:Released
    (Variables|/Script/Engine.CharacterMovementComponent|SetMaxWalkSpeed _charactermovement _running_speed)))

(event Input|ActionEvents|InputActionPlaceMagicCircle
  (params (Key :type Key%20Structure))
  ;[1 1 1] Place magic circle
  (:Pressed
    (if (Math|Boolean|ANDBoolean (Variables|Ability|GetCan%20Place%20Circle) (Variables|Default|GetIs%20Accepting%20Inputs) (not (AI|Components|NavMovement|IsFalling (Variables|Character|GetCharacterMovement))))
      (CallFunction|SetMovementandInputsEnabled false)
      (Variables|Ability|SetCan%20Place%20Circle false)
      (Variables|AnimationTrigger|SetPlacingCircle true)
      (Utilities|FlowControl|Delay 0.01)
      (Variables|AnimationTrigger|SetPlacingCircle false)
      (Utilities|FlowControl|Delay (Variables|Ability|GetDelay%20Before%20Circle%20Placement))
      (CallFunction|SummonMagicCircle)
      (Variables|ScanningInPrinterScanner|SetIs%20Circle%20Inside%20Scanner (Variables|ScanningInPrinterScanner|GetIs%20Player%20Inside%20Scanner))
      (Utilities|FlowControl|Delay (- (Variables|Ability|GetDelay%20Between%20Circle%20Placements) (Variables|Ability|GetDelay%20Before%20Circle%20Placement)))
      (Variables|Ability|SetCan%20Place%20Circle true)
      (CallFunction|SetMovementandInputsEnabled true))))

(event Input|ActionEvents|InputActionTeleportSpell
  (params (Key :type Key%20Structure))
  (bind _magic_circle (Variables|Default|GetMagic%20Circle))
  (bind _returnvalue (Transformation|GetActorLocation _magic_circle))
  (bind (_x _y _z) (Math|Vector|BreakVector _returnvalue))
  ;[1 1 1] Cast teleport spell
  (:Pressed
    (if (Math|Boolean|ANDBoolean (Variables|Ability|GetCan%20Teleport) (Variables|Default|GetIs%20Accepting%20Inputs) (Utilities|IsValid (Variables|Default|GetMagic%20Circle)))
      (CallFunction|SetMovementandInputsEnabled false)
      (Variables|Ability|SetCan%20Teleport false)
      (Variables|AnimationTrigger|SetTeleporting true)
      (Utilities|FlowControl|Delay 0.01)
      (Variables|AnimationTrigger|SetTeleporting false)
      (Utilities|FlowControl|Delay (Variables|Ability|GetDelay%20Before%20Teleport))
      (if (Variables|ScanningInPrinterScanner|GetIs%20Circle%20Inside%20Scanner) ; If the circle is inside the scanner and the scanner is closed, trigger a specific cinematic. Otherwise teleport as normal.
        (if (Variables|/Game/Placeables_Scenery/Scanner_BP.Scanner_BP_C|GetIs%20Scanner%20Closed (Variables|ScanningInPrinterScanner|GetScanner)) ; Only check scanner if scanner is present
          ;;[1 1 1] Reset state first due to not actually teleporting
          (Variables|Ability|SetCan%20Teleport true)
          (CallFunction|SetMovementandInputsEnabled true)
          (CallFunction|CutsceneStart)
          (Default|CallStartScanningCutscene) ; Dispatch event to level blueprint
          (Effects|SpawnEmitteratLocation "/Game/InfinityBladeEffects/Effects/FX_Combat_Base/Resurrection/P_Resurrection_02.P_Resurrection_02" (Transformation|GetActorLocation))
          (else
            (Transformation|Teleport (Math|Vector|MakeVector _x _y (+ _z (Variables|Ability|GetMagic%20Circle%20Offset))) "0, 0, 0" :!label _label)
            (Effects|SpawnEmitteratLocation "/Game/InfinityBladeEffects/Effects/FX_Combat_Base/Resurrection/P_Resurrection_02.P_Resurrection_02" (Transformation|GetActorLocation))
            (Utilities|FlowControl|Delay (- (Variables|Ability|GetDelay%20Between%20Teleports) (Variables|Ability|GetDelay%20Before%20Teleport)))
            (Variables|Ability|SetCan%20Teleport true)
            (CallFunction|SetMovementandInputsEnabled true)))
        (else
          (goto _label))))))

(event Input|ActionEvents|InputActionActivateObject
  (params (Key :type Key%20Structure))
  ;[1 1 1] Activate object (e.g. interact with a door)
  (:Pressed
    (if (Math|Boolean|ANDBoolean (Variables|Ability|GetCan%20Activate%20Object) (Variables|Default|GetIs%20Accepting%20Inputs) (not (AI|Components|NavMovement|IsFalling (Variables|Character|GetCharacterMovement))))
      (CallFunction|SetMovementandInputsEnabled false)
      (Variables|Ability|SetCan%20Activate%20Object false)
      (Variables|AnimationTrigger|SetActivatingObject true)
      (Utilities|FlowControl|Delay 0.01)
      (Variables|AnimationTrigger|SetActivatingObject false)
      (Utilities|FlowControl|Delay (Variables|Ability|GetDelay%20Before%20Activate%20Object))
      (CallFunction|TryActivateObject)
      (Utilities|FlowControl|Delay (- (Variables|Ability|GetDelay%20Between%20Activate%20Objects) (Variables|Ability|GetDelay%20Before%20Activate%20Object)))
      (Variables|Ability|SetCan%20Activate%20Object true)
      (CallFunction|SetMovementandInputsEnabled true))))

(fn ConstructionScript)

(fn SetMovementandInputsEnabled
  (params (Enabled :type Boolean))
  (bind _charactermovement (Variables|Character|GetCharacterMovement))
  (if Enabled
    (Pawn|Components|CharacterMovement|SetMovementMode _charactermovement "MOVE_Walking" 0)
    (Variables|Default|SetIs%20Accepting%20Inputs true)
    (else
      (Pawn|Components|CharacterMovement|DisableMovement _charactermovement)
      (Variables|Default|SetIs%20Accepting%20Inputs false)))
  (return))

(fn SummonMagicCircle
  (bind _returnvalue (Transformation|GetActorLocation))
  (bind _magic_circle_offset (Variables|Ability|GetMagic%20Circle%20Offset))
  (bind (_x _y _z) (Math|Vector|BreakVector _returnvalue))
  (bind _returnvalue_2 (- _z _magic_circle_offset))
  (bind _returnvalue_3 (Math|Vector|MakeVector _x _y _returnvalue_2))
  (if (Utilities|IsValid (Variables|Default|GetMagic%20Circle))
    (Transformation|Teleport (Variables|Default|GetMagic%20Circle) _returnvalue_3 "0, 0, 0")
    (else
      (bind _returnvalue_4 (Game|SpawnActorfromClass "/Game/Placeables_Scenery/MagicCircle_BP.MagicCircle_BP_C" (Math|Transform|MakeTransform _returnvalue_3 (Math|Conversions|RotationFromXVector (Math|Vector|VectorZero)) (Class|KismetMathLibrary|VectorOne)) "Undefined" 0 0))
      (Variables|Default|SetMagic%20Circle _returnvalue_4)))
  (return))

(fn TryActivateObject
  (bind _returnvalue (Transformation|GetActorLocation))
  (bind _outhit (Collision|LineTraceByChannel _returnvalue (+ _returnvalue (* (Transformation|GetActorForwardVector) (Variables|Default|GetActivate%20Trace%20Distance))) "TraceTypeQuery3" false 0 "None"))
  (Class|ActivatableI|Activate(Message) (.HitActor (Collision|BreakHitResult _outhit))))