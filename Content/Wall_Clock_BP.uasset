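; Wall clock actor whose hands show a preset time and tick forward during play.
; BeginPlay sets fixed starting rotations on the hour, minute and second hand pivots and records the next whole second of game time.
; Tick compares truncated game time to that counter, stepping the second and minute hands once per second.
; The hour hand deliberately stays still, keeping the displayed time roughly constant over long sessions.
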(event EventBeginPlay
  ;[1 1 1] Setup initial state
  (Transformation|SetRelativeRotation (Variables|Default|GetMinute%20Hand%20Pivot) "0,170.000000, 0" false false)
  (Transformation|SetRelativeRotation (Variables|Default|GetHour%20Hand%20Pivot) "0,255.000000, 0" false false)
  (Transformation|SetRelativeRotation (Variables|Default|GetSecond%20Hand%20Pivot) "0,40.000000, 0" false false)
  (Variables|Default|SetNext%20Second%20Since%20Start (Math|Float|Truncate (+ (Utilities|Time|GetTimeSeconds) 1.0))))

(event Collision|EventActorBeginOverlap
  (params (OtherActor :type Actor%20Object%20Reference)))

(event EventTick
  (params (DeltaSeconds :type Float%20%28single-precision%29))
  ;[1 1 1] Once per second, advance the hands. (Hour hand is ignored so even in the edge case of playing for hours, it still remains roughly the same time.)
  (if (> (Math|Float|Truncate (Utilities|Time|GetTimeSeconds)) (Variables|Default|GetNext%20Second%20Since%20Start))
    (Math|Integer|IncrementInt (Variables|Default|GetNext%20Second%20Since%20Start)
      (:%20%20
        (Transformation|AddRelativeRotation (Variables|Default|GetMinute%20Hand%20Pivot) (Math|Rotator|MakeRotator 0.0 0.0 0.1) false false)
        (Transformation|AddRelativeRotation (Variables|Default|GetSecond%20Hand%20Pivot) (Math|Rotator|MakeRotator 0.0 0.0 6.0) false false)))))

(fn ConstructionScript)