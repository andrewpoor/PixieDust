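; Desk fan scenery prop that constantly spins its blades and can be knocked off a desk onto the floor.
; Tick rotates the spinning parts around their roll axis at a set speed, scaled by delta time.
; GetKnockedOver chains two timelines without physics: one slides the actor by a locker-impact offset, then the next drops it by a floor offset while blending to an end rotation.
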(event Custom|Get%20Knocked%20Over
  ;[1 1 1] Get knocked off the desk and onto the floor
  (bind _alpha (Timeline|Get%20Knocked%20Into%20Locker PlayFromStart)
    (:Update
      (Transformation|SetActorLocation (Math|Vector|Lerp(Vector) (Variables|Default|GetCurrent%20Location) (+ (Variables|Default|GetCurrent%20Location) (Variables|Default|GetKnocked%20Into%20Locker%20Offset)) _alpha) false false))
    (:Finished
      (Variables|Default|SetCurrent%20Location (Transformation|GetActorLocation))
      (bind _alpha_2 (Timeline|Fall%20Down%20To%20Floor PlayFromStart)
        (:Update
          (Transformation|SetActorLocation (Math|Vector|Lerp(Vector) (Variables|Default|GetCurrent%20Location) (+ (Variables|Default|GetCurrent%20Location) (Variables|Default|GetFall%20To%20Floor%20Offset)) _alpha_2) false false)
          (Transformation|SetActorRotation (Math|Rotator|Lerp(Rotator) (Variables|Default|GetStarting%20Rotation) (Variables|Default|GetEnding%20Rotation) _alpha_2 true)))))))

(event EventBeginPlay
  ;[1 1 1] Setup variables
  (Variables|Default|SetCurrent%20Location (Transformation|GetActorLocation))
  (Variables|Default|SetStarting%20Rotation (Transformation|GetActorRotation)))

(event Collision|EventActorBeginOverlap
  (params (OtherActor :type Actor%20Object%20Reference)))

(event EventTick
  (params (DeltaSeconds :type Float%20%28single-precision%29))
  ;[1 1 1] Constantly spin the blades
  (Transformation|AddRelativeRotation (Variables|Default|GetSpinning%20Parts) (Math|Rotator|MakeRotator (* DeltaSeconds (Variables|Default|GetRotation%20Speed)) 0.0 0.0) false false))

(fn ConstructionScript)