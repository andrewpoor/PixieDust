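; Laptop scenery placeable that the player can open by interacting with it.
; An overlap box detects the PixieDustCharacter and shows a glow and an interact tutorial while the player is nearby.
; Activate disables both detection boxes, turns off the glow, and plays a timeline that rotates the hinge pivot from closed to open angle.
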(event OnComponentBeginOverlap(OverlapDetectionBox)
  (params (OverlappedComponent :type Primitive%20Component%20Object%20Reference) (OtherActor :type Actor%20Object%20Reference) (OtherComp :type Primitive%20Component%20Object%20Reference) (OtherBodyIndex :type Integer) (bFromSweep :type Boolean) (SweepResult :type Hit%20Result%20Structure%20%28by%20ref%29))
  ;[1 1 1] Glow when the player is nearby.
  (Utilities|Casting|CastToPixieDustCharacter OtherActor)
  (Components|Activation|Activate (Variables|Default|GetGlow) false)
  (Development|SetHiddeninGame (Variables|Default|GetInteract%20Tutorial) false false))

(event OnComponentEndOverlap(OverlapDetectionBox)
  (params (OverlappedComponent :type Primitive%20Component%20Object%20Reference) (OtherActor :type Actor%20Object%20Reference) (OtherComp :type Primitive%20Component%20Object%20Reference) (OtherBodyIndex :type Integer))
  ;[1 1 1] Glow when the player is nearby.
  (Utilities|Casting|CastToPixieDustCharacter OtherActor)
  (Components|Activation|Deactivate (Variables|Default|GetGlow))
  (Development|SetHiddeninGame (Variables|Default|GetInteract%20Tutorial) true false))

(event EventBeginPlay)

(event Collision|EventActorBeginOverlap
  (params (OtherActor :type Actor%20Object%20Reference)))

(event EventTick
  (params (DeltaSeconds :type Float%20%28single-precision%29)))

(event EventActivate
  ;[1 1 1] Activate by opening.
  (Collision|SetCollisionEnabled (Variables|Default|GetActivate%20Detection%20Box) "NoCollision")
  (Collision|SetCollisionEnabled (Variables|Default|GetOverlap%20Detection%20Box) "NoCollision")
  (Components|Activation|Deactivate (Variables|Default|GetGlow))
  (bind _alpha (Timeline|Laptop%20Opening Play)
    (:Update
      (Transformation|SetRelativeRotation (Variables|Default|GetHinge%20Pivot) (Math|Rotator|MakeRotator (Math|Float|Lerp (Variables|Default|GetClosed%20Angle) (Variables|Default|GetOpen%20Angle) _alpha) 0.0 0.0) false false))))

(fn ConstructionScript)