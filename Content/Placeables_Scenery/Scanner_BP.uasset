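; Interactive scanner prop with drawers that open once and buttons that open or close its lid.
; Overlap boxes make the nearby part glow and record it with the player for Activate to dispatch.
; Timelines slide the drawers after teleporting the player, or press the red or green button, then swing the hinged lid during a Pixie cutscene.
; A magic circle volume tells Pixie_BP when the player is inside the scanner.
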(event OnComponentBeginOverlap(DrawOverlapDetectionBox)
  (params (OverlappedComponent :type Primitive%20Component%20Object%20Reference) (OtherActor :type Actor%20Object%20Reference) (OtherComp :type Primitive%20Component%20Object%20Reference) (OtherBodyIndex :type Integer) (bFromSweep :type Boolean) (SweepResult :type Hit%20Result%20Structure%20%28by%20ref%29))
  ;[1 1 1] Draws glow when player is nearby
  (bind _aspixie_dust_character (Utilities|Casting|CastToPixieDustCharacter OtherActor))
  (Components|Activation|Activate (Variables|Default|GetDraw%20Glow) false)
  (Variables|Default|SetPart%20To%20Activate 1)
  (Variables|Default|SetActivating%20Player _aspixie_dust_character))

(event OnComponentEndOverlap(DrawOverlapDetectionBox)
  (params (OverlappedComponent :type Primitive%20Component%20Object%20Reference) (OtherActor :type Actor%20Object%20Reference) (OtherComp :type Primitive%20Component%20Object%20Reference) (OtherBodyIndex :type Integer))
  ;[1 1 1] Draws glow when player is nearby
  (Utilities|Casting|CastToPixieDustCharacter OtherActor)
  (Components|Activation|Deactivate (Variables|Default|GetDraw%20Glow))
  (Variables|Default|SetPart%20To%20Activate 0))

(event OnComponentBeginOverlap(ButtonsOverlapDetectionBox)
  (params (OverlappedComponent :type Primitive%20Component%20Object%20Reference) (OtherActor :type Actor%20Object%20Reference) (OtherComp :type Primitive%20Component%20Object%20Reference) (OtherBodyIndex :type Integer) (bFromSweep :type Boolean) (SweepResult :type Hit%20Result%20Structure%20%28by%20ref%29))
  ;[1 1 1] Buttons glow when player is nearby
  (bind _aspixie_dust_character (Utilities|Casting|CastToPixieDustCharacter OtherActor))
  (Components|Activation|Activate (Variables|Default|GetButtons%20Glow) false)
  (Variables|Default|SetPart%20To%20Activate 2)
  (Variables|Default|SetActivating%20Player _aspixie_dust_character))

(event OnComponentEndOverlap(ButtonsOverlapDetectionBox)
  (params (OverlappedComponent :type Primitive%20Component%20Object%20Reference) (OtherActor :type Actor%20Object%20Reference) (OtherComp :type Primitive%20Component%20Object%20Reference) (OtherBodyIndex :type Integer))
  ;[1 1 1] Buttons glow when player is nearby
  (Utilities|Casting|CastToPixieDustCharacter OtherActor)
  (Components|Activation|Deactivate (Variables|Default|GetButtons%20Glow))
  (Variables|Default|SetPart%20To%20Activate 0))

(event OnComponentBeginOverlap(MagicCircleDetectionBox)
  (params (OverlappedComponent :type Primitive%20Component%20Object%20Reference) (OtherActor :type Actor%20Object%20Reference) (OtherComp :type Primitive%20Component%20Object%20Reference) (OtherBodyIndex :type Integer) (bFromSweep :type Boolean) (SweepResult :type Hit%20Result%20Structure%20%28by%20ref%29))
  (bind _aspixie_bp (Utilities|Casting|CastToPixie_BP OtherActor))
  (Variables|/Game/Worlds_Characters/Overworld/OverworldPixieCharacter/Pixie_BP.Pixie_BP_C|SetIs%20Player%20Inside%20Scanner _aspixie_bp true)
  (Variables|/Game/Worlds_Characters/Overworld/OverworldPixieCharacter/Pixie_BP.Pixie_BP_C|SetScanner _aspixie_bp self))

(event OnComponentEndOverlap(MagicCircleDetectionBox)
  (params (OverlappedComponent :type Primitive%20Component%20Object%20Reference) (OtherActor :type Actor%20Object%20Reference) (OtherComp :type Primitive%20Component%20Object%20Reference) (OtherBodyIndex :type Integer))
  (bind _aspixie_bp (Utilities|Casting|CastToPixie_BP OtherActor))
  (Variables|/Game/Worlds_Characters/Overworld/OverworldPixieCharacter/Pixie_BP.Pixie_BP_C|SetIs%20Player%20Inside%20Scanner _aspixie_bp false))

(event EventBeginPlay
  (bind _top_draw (Variables|Default|GetTop%20Draw))
  (bind _bottom_draw (Variables|Default|GetBottom%20Draw))
  (bind _relativelocation (Variables|/Script/Engine.SceneComponent|GetRelativeLocation _top_draw))
  (bind _relativelocation_2 (Variables|/Script/Engine.SceneComponent|GetRelativeLocation _bottom_draw))
  ;[1 1 1] Set variables
  (Variables|Draws|SetTop%20Draw%20Closed%20Location _relativelocation)
  (Variables|Draws|SetTop%20Draw%20Open%20Location (+ _relativelocation (Variables|Draws|GetTop%20Draw%20Opened%20Offset)))
  (Variables|Draws|SetBottom%20Draw%20Start%20Location _relativelocation_2)
  (Variables|Draws|SetBottom%20Draw%20End%20Location (+ _relativelocation_2 (Variables|Draws|GetBottom%20Draw%20Opened%20Offset))))

(event Collision|EventActorBeginOverlap
  (params (OtherActor :type Actor%20Object%20Reference)))

(event EventTick
  (params (DeltaSeconds :type Float%20%28single-precision%29)))

(event EventActivate
  (bind _draw_activate_teleport_position (Variables|Default|GetDraw%20Activate%20Teleport%20Position))
  (switch int (Variables|Default|GetPart%20To%20Activate)
    (:Default
      ;[1 1 1] If anything else is activated, log an error
      (Development|PrintString "Error: Tried to activate scanner with nonexistant part not in list"))
    (:0
      (Development|PrintString "Error: Tried to activate scanner with nonexistant part 0"))
    (:1
      ;[1 1 1] Activate draws by opening them
      (Collision|SetCollisionEnabled (Variables|Default|GetDraw%20Activate%20Detection%20Box) "NoCollision")
      (Collision|SetCollisionEnabled (Variables|Default|GetDraw%20Overlap%20Detection%20Box) "NoCollision")
      (Components|Activation|Deactivate (Variables|Default|GetDraw%20Glow))
      (Transformation|Teleport (Variables|Default|GetActivating%20Player) (Transformation|GetWorldLocation _draw_activate_teleport_position) (Transformation|GetWorldRotation _draw_activate_teleport_position))
      (bind _alpha (Timeline|Draws%20opening PlayFromStart)
        (:Update
          (Transformation|SetRelativeLocation (Variables|Default|GetTop%20Draw) (Math|Vector|Lerp(Vector) (Variables|Draws|GetTop%20Draw%20Closed%20Location) (Variables|Draws|GetTop%20Draw%20Open%20Location) _alpha) false false)
          (Transformation|SetRelativeLocation (Variables|Default|GetBottom%20Draw) (Math|Vector|Lerp(Vector) (Variables|Draws|GetBottom%20Draw%20Start%20Location) (Variables|Draws|GetBottom%20Draw%20End%20Location) _alpha) false false))))
    (:2
      ;[1 1 1] Activate buttons by pressing one, then opening or closing the scanner
      (Collision|SetCollisionEnabled (Variables|Default|GetButtons%20Activate%20Detection%20Box) "NoCollision")
      (Collision|SetCollisionEnabled (Variables|Default|GetButtons%20Overlap%20Detection%20Box) "NoCollision")
      (Components|Activation|Deactivate (Variables|Default|GetButtons%20Glow))
      (bind _output_get (Variables|ButtonsandScannerLid|SetButton%20To%20Press (select (Variables|ButtonsandScannerLid|GetIs%20Scanner%20Closed) (Variables|Default|GetRed%20Button) (Variables|Default|GetGreen%20Button))))
      (Variables|ButtonsandScannerLid|SetButton%20Start%20Location (Variables|/Script/Engine.SceneComponent|GetRelativeLocation _output_get))
      (bind _alpha_2 (Timeline|Press%20Button PlayFromStart)
        (:Update
          (Transformation|SetRelativeLocation (Variables|ButtonsandScannerLid|GetButton%20To%20Press) (Math|Vector|Lerp(Vector) (Variables|ButtonsandScannerLid|GetButton%20Start%20Location) (+ (Variables|ButtonsandScannerLid|GetButton%20Start%20Location) (Variables|ButtonsandScannerLid|GetButton%20Pressed%20Offset)) _alpha_2) false false))
        (:Finished
          ;[1 1 1] Open or close the scanner in a cutscene
          (bind _aspixie_bp (Utilities|Casting|CastToPixie_BP (Variables|Default|GetActivating%20Player)))
          (Default|CutsceneStart _aspixie_bp)
          (if (Variables|ButtonsandScannerLid|GetIs%20Scanner%20Closed)
            (bind _alpha_3 (Timeline|Open%20or%20Close%20Scanner PlayFromStart)
              (:Update
                (Transformation|SetRelativeRotation (Variables|Default|GetHingePivot) (Math|Rotator|MakeRotator 0.0 (Math|Float|Lerp (Variables|ButtonsAndScannerLid|GetLid%20Start%20Angle) (Variables|ButtonsAndScannerLid|GetLid%20End%20Angle) _alpha_3) 0.0) false false))
              (:Finished
                (Collision|SetCollisionEnabled (Variables|Default|GetButtons%20Activate%20Detection%20Box) "QueryOnly")
                (Collision|SetCollisionEnabled (Variables|Default|GetButtons%20Overlap%20Detection%20Box) "QueryOnly")
                (Variables|ButtonsandScannerLid|SetIs%20Scanner%20Closed (not (Variables|ButtonsandScannerLid|GetIs%20Scanner%20Closed)))
                (bind _aspixie_bp_2 (Utilities|Casting|CastToPixie_BP (Variables|Default|GetActivating%20Player)))
                (Default|CutsceneFinished _aspixie_bp_2)))
            (else
              (Timeline|Open%20or%20Close%20Scanner ReverseFromEnd))))))))

(fn ConstructionScript)