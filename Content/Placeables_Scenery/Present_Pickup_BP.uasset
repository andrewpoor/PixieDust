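; Present pickup placeable that the Pixie player collects by touching it.
; On spawn it destroys itself if the PixieGameInstance already records this item as collected.
; Each tick the present mesh spins and bobs on a sine wave for emphasis.
; Overlapping its detection volume calls PickupItem on the Pixie, then spawns a particle burst and destroys the actor.
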(event OnComponentBeginOverlap(PickupDetection)
  (params (OverlappedComponent :type Primitive%20Component%20Object%20Reference) (OtherActor :type Actor%20Object%20Reference) (OtherComp :type Primitive%20Component%20Object%20Reference) (OtherBodyIndex :type Integer) (bFromSweep :type Boolean) (SweepResult :type Hit%20Result%20Structure%20%28by%20ref%29))
  ;[1 1 1] If the player touches the present, get picked up.
  (bind _aspixie_bp (Utilities|Casting|CastToPixie_BP OtherActor))
  (Default|PickupItem _aspixie_bp "NewEnumerator0")
  (CallFunction|GetPickedUp))

(event EventBeginPlay
  ;[1 1 1] When spawned, check if already picked up. If so, destroy this.
  (bind _aspixie_game_instance (Utilities|Casting|CastToPixieGameInstance (Game|GetGameInstance)))
  (if (Utilities|Enum|Equal(Enum) (Variables|/Game/PixieGameInstance.PixieGameInstance_C|GetCollected%20Item _aspixie_game_instance) "NewEnumerator0")
    (Actor|DestroyActor)))

(event EventTick
  (params (DeltaSeconds :type Float%20%28single-precision%29))
  ;[1 1 1] Make the present spin and float for emphasis
  (Transformation|AddLocalRotation (Variables|Default|GetPresent) (Math|Rotator|MakeRotator 0.0 0.0 (* (Variables|Default|GetSpin%20Rate) (Utilities|Time|GetWorldDeltaSeconds))) false false)
  (Transformation|SetRelativeLocation (Variables|Default|GetPresent) (Math|Vector|MakeVector 0.0 0.0 (* (Math|Trig|Sin(Degrees) (* (Variables|Default|GetFloating%20Oscillation%20Rate) (Utilities|Time|GetTimeSeconds))) (Variables|Default|GetFloating%20Displacement))) false false))

(fn ConstructionScript)

(fn GetPickedUp
  (bind _returnvalue (Transformation|GetActorTransform))
  (bind (_location _rotation _scale) (Math|Transform|BreakTransform _returnvalue))
  (Effects|SpawnEmitteratLocation "/Game/InfinityBladeEffects/Effects/FX_Combat_Base/Resurrection/P_Resurrection_02.P_Resurrection_02" _location _rotation _scale)
  (Actor|DestroyActor))