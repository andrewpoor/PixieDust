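; Falling statue scenery placeable that gets knocked off its edge when a toppleable book overlaps its capsule collider.
; On BeginPlay it records its start position and transform, sets its scale and derives a slip position offset along world X.
; The overlap plays a timeline that slides it to that point, then a second timeline lerps it to the floor position while pitching it over.
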(event OnComponentBeginOverlap(CapsuleCollider)
  (params (OverlappedComponent :type Primitive%20Component%20Object%20Reference) (OtherActor :type Actor%20Object%20Reference) (OtherComp :type Primitive%20Component%20Object%20Reference) (OtherBodyIndex :type Integer) (bFromSweep :type Boolean) (SweepResult :type Hit%20Result%20Structure%20%28by%20ref%29))
  (bind _slip_position (Variables|Default|GetSlip%20Position))
  (bind _fallen_floor_position (Variables|Default|GetFallen%20Floor%20Position))
  (bind (_x _y _z) (Math|Vector|BreakVector _slip_position))
  (bind (_x_2 _y_2 _z_2) (Math|Vector|BreakVector _fallen_floor_position))
  ;[1 1 1] When a book topples into this, fall off the edge. Start by slipping towards the edge (as pushed by the book).
  (Utilities|Casting|CastToToppleable_Book_Base OtherActor)
  (bind _alpha (Timeline|Slip%20Towards%20Edge Play)
    (:Update
      (Transformation|SetActorLocation (Math|Vector|Lerp(Vector) (Variables|Default|GetStarting%20Position) (Variables|Default|GetSlip%20Position) _alpha) false false))
    (:Finished
      ;[1 1 1] Now fall towards the floor.
      (bind (_direction _z_alpha _rotation_alpha _x_alpha) (Timeline|Fall%20To%20Floor Play)
        (:Update
          (Transformation|SetActorLocation (Math|Vector|MakeVector (Math|Float|Lerp _x _x_2 _x_alpha) _y_2 (Math|Float|Lerp _z _z_2 _z_alpha)) false false)
          (Transformation|SetActorRotation (Math|Rotator|MakeRotator 0.0 (Math|Float|Lerp (Variables|Default|GetUpright%20Angle) (Variables|Default|GetFallen%20Angle) _rotation_alpha) 0.0)))))))

(event EventBeginPlay
  ;[1 1 1] Setup variables
  (bind _output_get (Variables|Default|SetStarting%20Position (Transformation|GetActorLocation)))
  (Variables|Default|SetSlip%20Position (+ _output_get "45.000000, 0, 0"))
  (Variables|Default|SetStarting%20Transform (Transformation|GetActorTransform))
  (Transformation|SetActorScale3D (Variables|Default|GetStarting%20Scale)))

(event EventTick
  (params (DeltaSeconds :type Float%20%28single-precision%29)))

(fn ConstructionScript)

(fn GetStartingTransform
  (return (Variables|Default|GetStarting%20Transform)))