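; Scenery actor for a sleeping parent who is startled awake by either a ringing phone or the pixie's alarm.
; Each event plays skeletal mesh animations in sequence, timed by delays, then fires a dispatcher to notify the level blueprint.
; The phone sequence ends back in looping sleep, while the alarm sequence ends after looking at the clock.
; A separate event activates two dream glow effects, and waking toggles the first one's visibility.
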(event Custom|Phone%20Startles%20Awake
  ;[1 1 1] Animations for when the parent is startled awake by the phone ringing
  (Rendering|ToggleVisibility (Variables|Default|GetDream%20Glow%20FX%201) true) ; If glow FX is active, hide it.
  (Components|Animation|PlayAnimation (Variables|Default|GetSkeletal%20Mesh) "/Game/Placeables_Scenery/Parent/Animations/Parent_Anim_Parent_Wake_Up_1.Parent_Anim_Parent_Wake_Up_1" false)
  (Utilities|FlowControl|Delay (Variables|Default|GetWake%20Up%20From%20Phone%20Duration))
  (Components|Animation|PlayAnimation (Variables|Default|GetSkeletal%20Mesh) "/Game/Placeables_Scenery/Parent/Animations/Parent_Anim_Parent_Look_Around.Parent_Anim_Parent_Look_Around" false)
  (Utilities|FlowControl|Delay (Variables|Default|GetLook%20Around%20Duration))
  (Components|Animation|PlayAnimation (Variables|Default|GetSkeletal%20Mesh) "/Game/Placeables_Scenery/Parent/Animations/Parent_Anim_Parent_Back_To_Sleep.Parent_Anim_Parent_Back_To_Sleep" false)
  (Utilities|FlowControl|Delay (Variables|Default|GetBack%20To%20Sleep%20Duration))
  (Components|Animation|PlayAnimation (Variables|Default|GetSkeletal%20Mesh) "/Game/Placeables_Scenery/Parent/Animations/Parent_Anim_Parent_Sleeping.Parent_Anim_Parent_Sleeping" true)
  (Rendering|ToggleVisibility (Variables|Default|GetDream%20Glow%20FX%201) true) ; If glow FX is active, show it again.
  (Default|CallWakeUpfromPhoneAnimationFinished) ; Notify level blueprint
)

(event Custom|Activate%20Dream%20Glow
  (Components|Activation|Activate (Variables|Default|GetDream%20Glow%20FX%201) false)
  (Components|Activation|Activate (Variables|Default|GetDream%20Glow%20FX%202) false))

(event Custom|Alarm%20Startles%20Awake
  ;[1 1 1] Animations for when the parent is startled awake by the pixie's alarm
  (Rendering|ToggleVisibility (Variables|Default|GetDream%20Glow%20FX%201) true) ; If glow FX is active, hide it.
  (Components|Animation|PlayAnimation (Variables|Default|GetSkeletal%20Mesh) "/Game/Placeables_Scenery/Parent/Animations/Parent_Anim_Parent_Wake_Up_2.Parent_Anim_Parent_Wake_Up_2" false)
  (Utilities|FlowControl|Delay (Variables|Default|GetWake%20Up%20From%20Alarm%20Duration))
  (Components|Animation|PlayAnimation (Variables|Default|GetSkeletal%20Mesh) "/Game/Placeables_Scenery/Parent/Animations/Parent_Anim_Parent_Look_At_Clock.Parent_Anim_Parent_Look_At_Clock" false)
  (Utilities|FlowControl|Delay (Variables|Default|GetLook%20At%20Clock%20Duration))
  (Default|CallWakeUpfromAlarmAnimationFinished) ; Notify level blueprint
)

(event EventBeginPlay)

(event Collision|EventActorBeginOverlap
  (params (OtherActor :type Actor%20Object%20Reference)))

(event EventTick
  (params (DeltaSeconds :type Float%20%28single-precision%29)))

(fn ConstructionScript)