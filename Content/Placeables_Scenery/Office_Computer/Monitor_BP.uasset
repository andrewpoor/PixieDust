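; Office computer monitor prop that plays a scripted animation of the player's pixie being scanned onto the screen and escaping across the desktop.
; StartPlayerOnScreenAnimation notifies the connected scanner after scan-in, then chains flipbook swaps, landing sounds and timelines that lerp the sprite through falls and runs.
; The desktop fall lerps X linearly and Z on a curve for a gravity arc.
; It finally fires AnimationFinished for the level Blueprint and resets the sprite.
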(event Custom|Start%20Player%20On%20Screen%20Animation
  (bind _player_flipbook (Variables|Default|GetPlayer%20Flipbook))
  (bind _player_flipbook_2 (Variables|Default|GetPlayer%20Flipbook))
  (bind _player_flipbook_3 (Variables|Default|GetPlayer%20Flipbook))
  ;[1 1 1] Play scanning in animation, then fall to window floor
  (Sprite|SetFlipbook _player_flipbook "/Game/Placeables_Scenery/Office_Computer/Pixie_Scanning_Sprites/Flipbook_Pixie_Scanning_In.Flipbook_Pixie_Scanning_In")
  (Utilities|FlowControl|Delay (Class|PaperFlipbookComponent|GetFlipbookLength _player_flipbook))
  (Default|ScanningComplete (Variables|Default|GetConected%20Scanner))
  (Sprite|SetFlipbook (Variables|Default|GetPlayer%20Flipbook) "/Game/Worlds_Characters/PlatformerWorld/PlatformerPixieCharacter/Sprites/Flipbooks/Pixie_Midair_Flipbook.Pixie_Midair_Flipbook")
  (bind _alpha (Timeline|Fall%20Down%20To%20Window%20Floor PlayFromStart)
    (:Update
      (Transformation|SetWorldLocation (Variables|Default|GetPlayer%20Flipbook) (Math|Vector|Lerp(Vector) (Variables|Default|GetPlayer%20Flipbook%20Current%20Location) (+ (Variables|Default|GetPlayer%20Flipbook%20Current%20Location) (Variables|Default|GetOffset%20To%20Window%20Floor)) _alpha) false false))
    (:Finished
      ;[1 1 1] Land, then run to window edge
      (Audio|PlaySound2D "/Game/Audio/LittleRobotSoundFactory_SFX_Packs/Fantasy/270416__littlerobotsoundfactory__footstep-dirt-07.270416__littlerobotsoundfactory__footstep-dirt-07" 1.0 1.0 0.0 0 0) ; Sound of pixie landing
      (Sprite|SetFlipbook _player_flipbook_3 "/Game/Worlds_Characters/PlatformerWorld/PlatformerPixieCharacter/Sprites/Flipbooks/Pixie_Land_Flipbook.Pixie_Land_Flipbook")
      (Utilities|FlowControl|Delay (Class|PaperFlipbookComponent|GetFlipbookLength _player_flipbook_3))
      (Variables|Default|SetPlayer%20Flipbook%20Current%20Location (Transformation|GetWorldLocation (Variables|Default|GetPlayer%20Flipbook)))
      (Sprite|SetFlipbook (Variables|Default|GetPlayer%20Flipbook) "/Game/Worlds_Characters/PlatformerWorld/PlatformerPixieCharacter/Sprites/Flipbooks/Pixie_Run_Flipbook.Pixie_Run_Flipbook")
      (bind _alpha_2 (Timeline|Run%20To%20Window%20Edge PlayFromStart)
        (:Update
          (Transformation|SetWorldLocation (Variables|Default|GetPlayer%20Flipbook) (Math|Vector|Lerp(Vector) (Variables|Default|GetPlayer%20Flipbook%20Current%20Location) (+ (Variables|Default|GetPlayer%20Flipbook%20Current%20Location) (Variables|Default|GetOffset%20To%20Window%20Edge)) _alpha_2) false false))
        (:Finished
          ;[1 1 1] Fall out of window onto desktop floor
          (Sprite|SetFlipbook (Variables|Default|GetPlayer%20Flipbook) "/Game/Worlds_Characters/PlatformerWorld/PlatformerPixieCharacter/Sprites/Flipbooks/Pixie_Midair_Flipbook.Pixie_Midair_Flipbook")
          (Variables|Default|SetPlayer%20Flipbook%20Current%20Location (Transformation|GetWorldLocation (Variables|Default|GetPlayer%20Flipbook)))
          (bind (_direction _horizontal_alpha _vertical_alpha) (Timeline|Fall%20To%20Desktop%20Floor PlayFromStart)
            (:Update
              (Transformation|SetWorldLocation (Variables|Default|GetPlayer%20Flipbook) (Math|Vector|MakeVector (Math|Float|Lerp (.X (Math|Vector|BreakVector (Variables|Default|GetPlayer%20Flipbook%20Current%20Location))) (.X (Math|Vector|BreakVector (+ (Variables|Default|GetPlayer%20Flipbook%20Current%20Location) (Variables|Default|GetOffset%20To%20Desktop%20Floor)))) _horizontal_alpha) (.Y (Math|Vector|BreakVector (Variables|Default|GetPlayer%20Flipbook%20Current%20Location))) (Math|Float|Lerp (.Z (Math|Vector|BreakVector (Variables|Default|GetPlayer%20Flipbook%20Current%20Location))) (.Z (Math|Vector|BreakVector (+ (Variables|Default|GetPlayer%20Flipbook%20Current%20Location) (Variables|Default|GetOffset%20To%20Desktop%20Floor)))) _vertical_alpha)) false false))
            (:Finished
              ;[1 1 1] Land, then run off-screen (by running behind the chat box window)
              (Audio|PlaySound2D "/Game/Audio/LittleRobotSoundFactory_SFX_Packs/Fantasy/270416__littlerobotsoundfactory__footstep-dirt-07.270416__littlerobotsoundfactory__footstep-dirt-07" 1.0 1.0 0.0 0 0) ; Sound of pixie landing
              (Sprite|SetFlipbook _player_flipbook_2 "/Game/Worlds_Characters/PlatformerWorld/PlatformerPixieCharacter/Sprites/Flipbooks/Pixie_Land_Flipbook.Pixie_Land_Flipbook")
              (Utilities|FlowControl|Delay (Class|PaperFlipbookComponent|GetFlipbookLength _player_flipbook_2))
              (Variables|Default|SetPlayer%20Flipbook%20Current%20Location (Transformation|GetWorldLocation (Variables|Default|GetPlayer%20Flipbook)))
              (Sprite|SetFlipbook (Variables|Default|GetPlayer%20Flipbook) "/Game/Worlds_Characters/PlatformerWorld/PlatformerPixieCharacter/Sprites/Flipbooks/Pixie_Run_Flipbook.Pixie_Run_Flipbook")
              (bind _alpha_3 (Timeline|Run%20To%20Screen%20Edge PlayFromStart)
                (:Update
                  (Transformation|SetWorldLocation (Variables|Default|GetPlayer%20Flipbook) (Math|Vector|Lerp(Vector) (Variables|Default|GetPlayer%20Flipbook%20Current%20Location) (+ (Variables|Default|GetPlayer%20Flipbook%20Current%20Location) (Variables|Default|GetOffset%20To%20Screen%20Edge)) _alpha_3) false false))
                (:Finished
                  (Default|CallAnimationFinished) ; Once finished, notify the level blueprint
                  (CallFunction|Reset))))))))))

(event Custom|Reset
  ;[1 1 1] Reset pixie so animation can start again
  (bind _output_get (Variables|Default|SetPlayer%20Flipbook%20Current%20Location (Variables|Default|GetPlayer%20Flipbook%20Starting%20Position)))
  (Transformation|SetWorldLocation (Variables|Default|GetPlayer%20Flipbook) _output_get false false)
  (Sprite|SetFlipbook (Variables|Default|GetPlayer%20Flipbook)))

(event EventBeginPlay
  ;[1 1 1] Setup variables
  (bind _output_get (Variables|Default|SetPlayer%20Flipbook%20Starting%20Position (Transformation|GetWorldLocation (Variables|Default|GetPlayer%20Flipbook))))
  (Variables|Default|SetPlayer%20Flipbook%20Current%20Location _output_get))

(event Collision|EventActorBeginOverlap
  (params (OtherActor :type Actor%20Object%20Reference)))

(event EventTick
  (params (DeltaSeconds :type Float%20%28single-precision%29)))

(fn ConstructionScript)