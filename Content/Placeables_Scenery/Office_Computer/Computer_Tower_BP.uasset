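; Placeable office computer tower scenery with a hinged flap and a designated player spawn point.
; ToggleFlapOpenOrClosed plays or reverses a timeline that interpolates the hinge between closed and open rotations, flipping the closed-state flag when the timeline finishes.
; A getter exposes the spawn point component's world location and rotation to callers.
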(event Custom|Toggle%20Flap%20Open%20Or%20Closed
  (if (Variables|Default|GetFlap%20Closed)
    (bind _alpha (Timeline|Open%20Flap PlayFromStart)
      (:Update
        (Transformation|SetRelativeRotation (Variables|Default|GetFlap%20Hinge) (Math|Rotator|Lerp(Rotator) (Variables|Default|GetFlap%20Closed%20Rotation) (Variables|Default|GetFlap%20Open%20Rotation) _alpha true) false false))
      (:Finished
        (Variables|Default|SetFlap%20Closed (not (Variables|Default|GetFlap%20Closed)))))
    (else
      (Timeline|Open%20Flap ReverseFromEnd))))

(event EventBeginPlay)

(event Collision|EventActorBeginOverlap
  (params (OtherActor :type Actor%20Object%20Reference)))

(event EventTick
  (params (DeltaSeconds :type Float%20%28single-precision%29)))

(fn ConstructionScript)

(fn GetPlayerSpawnLocationandRotation
  (bind _player_spawn_point (Variables|Default|GetPlayer%20Spawn%20Point))
  (return (Transformation|GetWorldLocation _player_spawn_point) (Transformation|GetWorldRotation _player_spawn_point)))