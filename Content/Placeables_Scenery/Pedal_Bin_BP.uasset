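; Pedal bin scenery placeable that acts as a launcher, flipping its lid when a Falling_Statue_BP hits the pedal's impact box.
; A detection box tracks whether the Pixie player stands on the lid and mirrors that state onto the player.
; On impact, a standing player is teleported to a launch point while a timeline rotates pedal and lid, then launched via LaunchPixie when it finishes.
; It also stores its starting transform for external retrieval.
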(event OnComponentBeginOverlap(ImpactDetectionBox)
  (params (OverlappedComponent :type Primitive%20Component%20Object%20Reference) (OtherActor :type Actor%20Object%20Reference) (OtherComp :type Primitive%20Component%20Object%20Reference) (OtherBodyIndex :type Integer) (bFromSweep :type Boolean) (SweepResult :type Hit%20Result%20Structure%20%28by%20ref%29))
  (bind _launch_location (Variables|Default|GetLaunch%20Location))
  ;[1 1 1] Flip the lid open when the pedal is pressed by the falling statue.
  (Utilities|Casting|CastToFalling_Statue_BP OtherActor)
  (if (Variables|Default|GetIs%20Player%20On%20Lid)
    (Transformation|Teleport (Variables|Default|GetPlayer) (Transformation|GetWorldLocation _launch_location) (Transformation|GetWorldRotation _launch_location)))
  (Utilities|FlowControl|Delay 0.01)
  (bind _alpha (Timeline|Press%20Pedal%20and%20Open%20Lid Play)
    (:Update
      (Transformation|SetRelativeRotation (Variables|Default|GetPedal%20Base) (Math|Rotator|MakeRotator 0.0 (Math|Float|Lerp (Variables|Default|GetPedal%20Neutral%20Angle) (Variables|Default|GetPedel%20Pressed%20Angle) _alpha) 0.0) false false)
      (Transformation|SetRelativeRotation (Variables|Default|GetLid%20Pivot) (Math|Rotator|MakeRotator 0.0 (Math|Float|Lerp (Variables|Default|GetLid%20Closed%20Angle) (Variables|Default|GetLid%20Opened%20Angle) _alpha) 0.0) false false))
    (:Finished
      (if (Variables|Default|GetIs%20Player%20On%20Lid)
        (Default|LaunchPixie (Variables|Default|GetPlayer) (Variables|Default|GetPlayer%20Launch%20Velocity) (Variables|Default|GetPlayer%20Flight%20Duration) true false)))))

(event OnComponentBeginOverlap(PlayerDetectionBox)
  (params (OverlappedComponent :type Primitive%20Component%20Object%20Reference) (OtherActor :type Actor%20Object%20Reference) (OtherComp :type Primitive%20Component%20Object%20Reference) (OtherBodyIndex :type Integer) (bFromSweep :type Boolean) (SweepResult :type Hit%20Result%20Structure%20%28by%20ref%29))
  ;[1 1 1] Detect if the player is standing on the lid.
  (bind _aspixie_bp (Utilities|Casting|CastToPixie_BP OtherActor))
  (Variables|Default|SetPlayer _aspixie_bp)
  (Variables|Default|SetIs%20Player%20On%20Lid true)
  (Variables|/Game/Worlds_Characters/Overworld/OverworldPixieCharacter/Pixie_BP.Pixie_BP_C|SetIs%20On%20Bin%20Lid _aspixie_bp true))

(event OnComponentEndOverlap(PlayerDetectionBox)
  (params (OverlappedComponent :type Primitive%20Component%20Object%20Reference) (OtherActor :type Actor%20Object%20Reference) (OtherComp :type Primitive%20Component%20Object%20Reference) (OtherBodyIndex :type Integer))
  ;[1 1 1] Detect if the player is standing on the lid.
  (bind _aspixie_bp (Utilities|Casting|CastToPixie_BP OtherActor))
  (Variables|Default|SetIs%20Player%20On%20Lid false)
  (Variables|/Game/Worlds_Characters/Overworld/OverworldPixieCharacter/Pixie_BP.Pixie_BP_C|SetIs%20On%20Bin%20Lid _aspixie_bp false))

(event EventBeginPlay
  (Variables|Default|SetStarting%20Transform (Transformation|GetActorTransform)))

(event Collision|EventActorBeginOverlap
  (params (OtherActor :type Actor%20Object%20Reference)))

(event EventTick
  (params (DeltaSeconds :type Float%20%28single-precision%29)))

(fn ConstructionScript)

(fn GetStartingTransform
  (return (Variables|Default|GetStarting%20Transform)))